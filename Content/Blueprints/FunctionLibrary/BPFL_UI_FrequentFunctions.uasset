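; Blueprint function library of shared UI helpers that let callers push and remove widgets without holding a UI reference.
; Push, remove, prompt and transition calls fetch the UI base from the given PlayerController and forward to it; all but prompt print if it is invalid.
; Push-to-all delegates to GS_GameState's TransitionTest.
; The cursor helper sets mouse visibility on every valid controller in the GameState's PlayerArray.
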(fn `Game_PushPromptWidget`
  (params (`Prompt Base Class` :type "CommonActivatableWidget Class Reference") (`In Prompt Text` :type Text) (`In Prompt Index` :type Integer) (`Widget Owner` :type "Widget Object Reference") (`Player Controller` :type "PlayerController Object Reference"))
  (bind _wbp_user_base_game (message `/Game/Blueprints/Data/Interface/BPI_Controller.Fn_GetUIBase` `Player Controller`))
  (`/Engine/EditorBlueprintResources/StandardMacros.IsValid` _wbp_user_base_game
    (:`Is Valid`
      (`/Game/Blueprints/UI/WBP_UI_Base.PushPrompt` _wbp_user_base_game (`local.Prompt Base Class`) (`local.In Prompt Text`) (`local.In Prompt Index`) (`local.Widget Owner`)))))

(fn `Game_PushTransitionWidget`
  (params (`Controller to Edit` :type "Controller Object Reference") (`Widget Class` :type "CommonActivatableWidget Class Reference") (`Entry?` :type Boolean))
  ;[1 1 1] Using a function library for push widgets so anything can push without needing a reference to the UI
  (bind _wbp_user_base_game (message `/Game/Blueprints/Data/Interface/BPI_Controller.Fn_GetUIBase` `Controller to Edit`))
  (`/Engine/EditorBlueprintResources/StandardMacros.IsValid` _wbp_user_base_game
    (:`Is Valid`
      (`/Game/Blueprints/UI/WBP_UI_Base.PushTransition` _wbp_user_base_game `Widget Class` (`local.Entry?`)))
    (:`Is Not Valid`
      (`KismetSystemLibrary.PrintString` null "UI base on PlayerController is not valid" true true (struct :`R` 1.0 :`B` 0.149247 :`A` 1.0) 30.0 "GetUIBASE"))))

(fn `Game_PushWidget`
  (params (`Controller to Edit` :type "Controller Object Reference") (`Widget Slot` :type "/Game/Blueprints/Data/Enumeration/Enum_WidgetSlot Enum" :default "NewEnumerator0") (`Widget Class` :type "CommonActivatableWidget Class Reference"))
  (returns (`Returned Widget` :type "CommonActivatableWidget Object Reference"))
  ;[1 1 1] Using a function library for push widgets so anything can push without needing a reference to the UI
  (bind _wbp_user_base_game (message `/Game/Blueprints/Data/Interface/BPI_Controller.Fn_GetUIBase` `Controller to Edit`))
  (`/Engine/EditorBlueprintResources/StandardMacros.IsValid` _wbp_user_base_game
    (:`Is Valid`
      (bind _returnvalue (`/Game/Blueprints/UI/WBP_UI_Base.PushWidget` _wbp_user_base_game `Widget Slot` `Widget Class` false))
      (return _returnvalue))
    (:`Is Not Valid`
      (`KismetSystemLibrary.PrintString` null (`KismetTextLibrary.Conv_TextToString` (`|FormatText` "UI base on PlayerController is not valid: Owner: {a}" `Controller to Edit`)) true true (struct :`R` 1.0 :`B` 0.149247 :`A` 1.0) 30.0 "GetUIBASE"))))

(fn `Game_RemoveWidget`
  (params (`Controller to Edit` :type "Controller Object Reference") (`Widget Slot` :type "/Game/Blueprints/Data/Enumeration/Enum_WidgetSlot Enum" :default "NewEnumerator0") (Widget :type "CommonActivatableWidget Object Reference"))
  ;[1 1 1] Using a function library for push widgets so anything can push without needing a reference to the UI
  (bind _wbp_user_base_game (message `/Game/Blueprints/Data/Interface/BPI_Controller.Fn_GetUIBase` `Controller to Edit`))
  (`/Engine/EditorBlueprintResources/StandardMacros.IsValid` _wbp_user_base_game
    (:`Is Valid`
      (`/Game/Blueprints/UI/WBP_UI_Base.RemoveWidget` _wbp_user_base_game `Widget Slot` Widget))
    (:`Is Not Valid`
      (`KismetSystemLibrary.PrintString` null "UI base on PlayerController is not valid" true true (struct :`R` 1.0 :`B` 0.149247 :`A` 1.0) 30.0 "GetUIBASE"))))

(fn `Online_PushWidgetToAll`
  (params (`Widget Slot` :type "/Game/Blueprints/Data/Enumeration/Enum_WidgetSlot Enum" :default "NewEnumerator0") (`Widget Class` :type "CommonActivatableWidget Class Reference"))
  (bind _asgs_game_state (cast `/Game/Blueprints/GameMode/GS_GameState` (`GameplayStatics.GetGameState` null)))
  (`/Game/Blueprints/GameMode/GS_GameState_Vs.Transition Test` _asgs_game_state `Widget Slot` `Widget Class`))

(fn `UI_ShowMouse_Cursor`
  (params (`Enable Mouse?` :type Boolean))
  (for _array_element (`GameStateBase.PlayerArray` (`GameplayStatics.GetGameState` null))
    (bind _returnvalue (`PlayerState.GetPlayerController` _array_element))
    (`/Engine/EditorBlueprintResources/StandardMacros.IsValid` _returnvalue
      (:`Is Valid`
        (set `PlayerController.bShowMouseCursor` (`local.Enable Mouse?`) _returnvalue)))))