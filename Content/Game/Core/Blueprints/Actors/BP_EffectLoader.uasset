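; BP_EffectLoader is a short-lived actor that loads sets of materials and Niagara effects into the scene, apparently to warm them up.
; On BeginPlay it adds a static mesh component for each material in MatsToLoad and a Niagara component for each system in EffectsToLoad.
; After a brief delay it destroys itself, taking the temporary components with it.
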(event `self.ReceiveBeginPlay`
  (`|ExecutionSequence`
    (:`then_0`
      (bind _result (`BlueprintSetLibrary.Set_ToArray` (`self.MatsToLoad`)))
      (for _array_element _result
        (bind _returnvalue (`AddComponent|NODE_AddStaticMeshComponent-0`))
        (`PrimitiveComponent.SetMaterial` _returnvalue 0 _array_element)))
    (:`then_1`
      (bind _result_2 (`BlueprintSetLibrary.Set_ToArray` (`self.EffectsToLoad`)))
      (for _array_element_2 _result_2
        (bind _returnvalue_2 (`AddComponent|NODE_AddNiagaraComponent-0`))
        (`NiagaraComponent.SetAsset` _returnvalue_2 _array_element_2 true))
      (`KismetSystemLibrary.Delay` 5.0)
      (`self.K2_DestroyActor`))))

(fn `UserConstructionScript`)