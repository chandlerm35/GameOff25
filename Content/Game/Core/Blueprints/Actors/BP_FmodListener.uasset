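; FMOD listener actor that turns music parameter changes into rhythm events on GI_GameInstance, which it caches at BeginPlay.
; Each Tick it reads and debug-prints the global "BossTriggers" parameter, calling RhythmTempo when the value nears one.
; A gate closes after each call and reopens at zero or below, preventing repeat triggers on one beat.
; Similar logic for RhythmBeat and BossMove is present but unhooked.
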(event `self.ReceiveBeginPlay`
  (`self.Initialize`))

(event `self.ReceiveTick`
  (params (DeltaSeconds :type "Float (single-precision)"))
  (bind (_uservalue _finalvalue) (`FMODBlueprintStatics.GetGlobalParameterValueByName` "BossTriggers"))
  (`KismetSystemLibrary.PrintString` (`KismetTextLibrary.Conv_TextToString` (`|FormatText` "BossTrigger: {rhythm_tempo} \n" _finalvalue)) true true (struct :`G` 0.66 :`B` 1.0 :`A` 1.0) 2.0 "Tempo")
  (`|ExecutionSequence`
    (:`then_0`
      ; Rhythm Tempo
      (if (>= _finalvalue 0.98)
        (`/Engine/EditorBlueprintResources/StandardMacros.Gate` true :!label _label ; Prevents multiple triggers on one beat
          (:`Exit`
            (`/Game/Game/Core/GameInstance/GI_GameInstance.Rhythm_tempo` (`self.GameInstance`))
            (goto _label :!via `Close`)))
        (elif (<= _finalvalue 0.0)
          (goto _label :!via `Open`))))))

(fn `Initialize`
  (bind _asgi_game_instance (cast `/Game/Game/Core/GameInstance/GI_GameInstance` (`GameplayStatics.GetGameInstance`))
    (:`then`
      (set `self.GameInstance` _asgi_game_instance))
    (:`CastFailed`
      (`KismetSystemLibrary.PrintString` (`KismetTextLibrary.Conv_TextToString` (`|FormatText` "{Class} class memeber {display} failed to cast to Game Instance" (`KismetSystemLibrary.GetClassDisplayName` (`GameplayStatics.GetObjectClass` self)) (`KismetSystemLibrary.GetDisplayName` self)))))))

(fn `UserConstructionScript`)