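; BP_OverlapTrigger is a box trigger volume that sends OnTriggerMessage to an assigned ActorToTrigger when the player's pawn enters it.
; On BeginPlay its text component displays the configurable TriggerText.
; A Gate closes after firing to block repeat messages during an overlap.
; When the player leaves, the gate reopens if Retriggerable is set; otherwise the trigger destroys itself.
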(event `self.ReceiveBeginPlay`
  (`TextRenderComponent.K2_SetText` (`self.text`) (`self.TriggerText`)))

(event `self.Box.OnComponentBeginOverlap`
  (params (OverlappedComponent :type "PrimitiveComponent Object Reference") (OtherActor :type "Actor Object Reference") (OtherComp :type "PrimitiveComponent Object Reference") (OtherBodyIndex :type Integer) (bFromSweep :type Boolean) (SweepResult :type "HitResult Structure (by ref)"))
  (if (== (`GameplayStatics.GetPlayerPawn` 0) OtherActor)
    (`/Engine/EditorBlueprintResources/StandardMacros.Gate` false :!label _label
      (:`Exit`
        (message `/Game/Game/Core/Blueprints/Data/Interface/BPI_Triggerable.OnTrigger` (`self.ActorToTrigger`))
        (goto _label :!via `Close`)))))

(event `self.Box.OnComponentEndOverlap`
  (params (OverlappedComponent :type "PrimitiveComponent Object Reference") (OtherActor :type "Actor Object Reference") (OtherComp :type "PrimitiveComponent Object Reference") (OtherBodyIndex :type Integer))
  (if (== (`GameplayStatics.GetPlayerPawn` 0) OtherActor)
    (if (`self.Retriggerable?`)
      (goto _label :!via `Open`)
      (else
        (`self.K2_DestroyActor`)))))

(fn `UserConstructionScript`)