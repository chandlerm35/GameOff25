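; BP_PooledActor is an actor meant for object pooling, switched between active and dormant states instead of being spawned and destroyed.
; SetInUse toggles collision, visibility and tick together, and each instance starts dormant on BeginPlay.
; On activation it restarts a time-to-live timer that calls ReturnToPool, which deactivates and hides the actor for reuse.
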(event `self.ReceiveBeginPlay`
  ;[1 1 1] Pooled Objects begin not in use.
  (`self.SetInUse` false))

(event `SetInUse`
  (params (InUse :type Boolean))
  (set `self.InUse` InUse)
  (`self.SetActorEnableCollision` InUse)
  (`self.SetActorHiddenInGame` (not InUse))
  (`self.SetActorTickEnabled` InUse)
  ;[1 1 1] Clears timer before making a new one
  (`KismetSystemLibrary.K2_ClearAndInvalidateTimerHandle` (`self.TimeToLiveTimer`))
  (if InUse
    (bind _returnvalue (`KismetSystemLibrary.K2_SetTimerDelegate` (delegate `ReturnToPool`) (`self.TimeToLive`)))
    (set `self.TimeToLiveTimer` _returnvalue)))

(event `ReturnToPool`
  (`self.SetInUse` false)
  (`self.SetActorHiddenInGame` true))

(fn `UserConstructionScript`)