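; Base projectile actor that applies Gameplay Ability System damage on impact and then returns to a pool.
; A Box hit prints the actor's name and calls OnProjectileImpact, then applies the stored effect spec to any ability system on that actor, with a hardcoded SetByCaller Data.Damage magnitude.
; The construction script feeds Speed and MaxSpeed into ProjectileMovement; the ApplyDamage function is an empty stub.
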(event `self.Box.OnComponentHit`
  (params (HitComponent :type "PrimitiveComponent Object Reference") (OtherActor :type "Actor Object Reference") (OtherComp :type "PrimitiveComponent Object Reference") (NormalImpulse :type "Vector Structure") (Hit :type "HitResult Structure (by ref)"))
  (bind _returnvalue (`AbilitySystemBlueprintLibrary.GetAbilitySystemComponent` OtherActor))
  (`KismetSystemLibrary.PrintString` (`KismetSystemLibrary.GetDisplayName` OtherActor) true true (struct :`G` 0.66 :`B` 1.0 :`A` 1.0) 50.0)
  (`self.OnProjectileImpact` OtherActor Hit)
  (`|ExecutionSequence`
    (:`then_0`
      (`/Engine/EditorBlueprintResources/StandardMacros.IsValid` _returnvalue ; Does hit actor have ability system?
        (:`Is Valid`
          (bind _returnvalue_2 (`AbilitySystemBlueprintLibrary.AssignTagSetByCallerMagnitude` (`self.SpecHandle`) (struct :`TagName` "Data.Damage") -10.0))
          (`AbilitySystemComponent.BP_ApplyGameplayEffectSpecToSelf` _returnvalue _returnvalue_2))))
    (:`then_1`
      (`self.ReturnToPool`))))

(fn `ApplyDamage`)

(fn `UserConstructionScript`
  (bind _projectilemovement (`self.ProjectileMovement`))
  (`parent.UserConstructionScript`)
  (set `ProjectileMovementComponent.InitialSpeed` (`self.Speed`) _projectilemovement)
  (set `ProjectileMovementComponent.MaxSpeed` (`self.MaxSpeed`) _projectilemovement))