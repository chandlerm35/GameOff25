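; BP_Shield is a shield actor whose static mesh scales in on activation and scales out before being removed.
; Activate makes the mesh visible and plays a timeline that drives its relative scale uniformly.
; Deactivate runs a second timeline in reverse from its end to drive the scale, then destroys the actor when finished.
; SetMaterial lets a caller swap the mesh's material.
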(event `Activate`
  (`SceneComponent.SetVisibility` (`self.StaticMesh`) true false)
  (bind (_direction _newtrack_0) (`Timeline|Timeline` :!via `PlayFromStart`)
    (:`Update`
      (`SceneComponent.SetRelativeScale3D` (`self.StaticMesh`) (`KismetMathLibrary.Conv_DoubleToVector` _newtrack_0)))))

(event `Deactivate`
  (bind (_direction _newtrack_0) (`Timeline|Timeline_0` :!via `ReverseFromEnd`)
    (:`Update`
      (`SceneComponent.SetRelativeScale3D` (`self.StaticMesh`) (`KismetMathLibrary.Conv_DoubleToVector` _newtrack_0)))
    (:`Finished`
      (`self.K2_DestroyActor`))))

(event `SetMaterial`
  (params (`Material Instance` :type "MaterialInstance Object Reference"))
  (`PrimitiveComponent.SetMaterial` (`self.StaticMesh`) 0 `Material Instance`))

(fn `UserConstructionScript`)