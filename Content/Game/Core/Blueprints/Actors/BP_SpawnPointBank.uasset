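; Spawn point bank actor that groups nine individual spawn point references and raises spawn requests when triggered.
; UpdateSpawnPointArray appends the nine references to the SpawnPoints array without clearing it, then broadcasts BanksArrayUpdated.
; OnTrigger broadcasts RequestSpawn with the bank itself as payload, leaving the actual spawning to listeners.
; A delayed test request with a debug print is left disconnected, and BeginPlay does nothing.
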(event `self.ReceiveBeginPlay`)

(event `/Game/Game/Core/Blueprints/Data/Interface/BPI_Triggerable.OnTrigger`
  (`self.RequestSpawn` self))

(fn `UpdateSpawnPointArray`
  (bind _spawnpoints (`self.SpawnPoints`))
  (`KismetArrayLibrary.Array_Add` _spawnpoints (`self.SpawnPoint1`))
  (`KismetArrayLibrary.Array_Add` _spawnpoints (`self.SpawnPoint2`))
  (`KismetArrayLibrary.Array_Add` _spawnpoints (`self.SpawnPoint3`))
  (`KismetArrayLibrary.Array_Add` _spawnpoints (`self.SpawnPoint4`))
  (`KismetArrayLibrary.Array_Add` _spawnpoints (`self.SpawnPoint5`))
  (`KismetArrayLibrary.Array_Add` _spawnpoints (`self.SpawnPoint6`))
  (`KismetArrayLibrary.Array_Add` _spawnpoints (`self.SpawnPoint7`))
  (`KismetArrayLibrary.Array_Add` _spawnpoints (`self.SpawnPoint8`))
  (`KismetArrayLibrary.Array_Add` _spawnpoints (`self.SpawnPoint9`))
  (`self.BanksArrayUpdated`))

(fn `UserConstructionScript`)