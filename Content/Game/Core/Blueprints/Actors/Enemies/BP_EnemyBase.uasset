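; BP_EnemyBase is a base enemy actor that takes damage through a BPCDamageSystem component.
; TakeDamage forwards damage info to the component, whose death and damage-response events are bound in the Construction Script to handlers that only print debug messages.
; GetCurrentHealth, GetMaxHealth and Heal are stubs returning zero.
; A DamageTest event applies fixed damage, but its looping timer is disconnected and never runs.
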(event `self.ReceiveBeginPlay`)

(event `DamageTest`
  ; DAMAGE TEST
  (`self.TakeDamage` (make `/Game/Game/Core/Blueprints/Data/Structs/S_DamageInfo` 25.0)))

(event `/Game/Game/Core/Blueprints/Data/Interface/BPI_Damageable.Death`
  ; Fires on HP reaching zero
  (`KismetSystemLibrary.PrintString` (`KismetTextLibrary.Conv_TextToString` (`|FormatText` "{actor} has died" (`KismetTextLibrary.Conv_StringToText` (`KismetSystemLibrary.GetDisplayName` self)))) true true (struct :`R` 1.0 :`B` 0.119528 :`A` 1.0) 5.0))

(event `DamageResponse`
  ; Fires when damaged
  (`KismetSystemLibrary.PrintString` (`KismetTextLibrary.Conv_TextToString` (`|FormatText` "{actor} has been damaged" (`KismetTextLibrary.Conv_StringToText` (`KismetSystemLibrary.GetDisplayName` self)))) true true (struct :`R` 1.0 :`B` 0.103232 :`A` 1.0) 5.0))

(fn `GetCurrentHealth`
  (returns (Health :type "Float (double-precision)"))
  (return 0.0))

(fn `GetMaxHealth`
  (returns (MaxHealth :type "Float (double-precision)"))
  (return 0.0))

(fn `Heal`
  (params (Amount :type "Float (double-precision)"))
  (returns (NewHealth :type "Float (double-precision)"))
  (return 0.0))

(fn `TakeDamage`
  (params (DamageInfo :type "/Game/Game/Core/Blueprints/Data/Structs/S_DamageInfo Structure"))
  (`/Game/Game/Core/Blueprints/Components/BPC_DamageSystem.TakeDamage` (`self.BPC_DamageSystem`) DamageInfo))

(fn `UserConstructionScript`
  (bind _bpc_damagesystem (`self.BPC_DamageSystem`))
  (add `/Game/Game/Core/Blueprints/Components/BPC_DamageSystem.OnDeath` _bpc_damagesystem (`|CreateDelegate` :!event `Death`))
  (add `/Game/Game/Core/Blueprints/Components/BPC_DamageSystem.OnDamageResponse` _bpc_damagesystem (`|CreateDelegate` :!event `DamageResponse`)))