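; Base pooled projectile that flies homing or straight at a target actor and deals damage through the Gameplay Ability System.
; FireProjectile plays a spawn cue, then sets the homing component or aims velocity at the target.
; Sphere overlap with non-instigators signals impact and applies GE_DamageInstant on authority, with damage set by caller.
; Overlaps and blocking hits return it to the pool with an impact gameplay cue.
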(event `self.ReceiveBeginPlay`
  (`parent.ReceiveBeginPlay`)
  (`PrimitiveComponent.IgnoreActorWhenMoving` (`self.Sphere`) (`self.GetOwner`) false))

(event `self.Sphere.OnComponentBeginOverlap`
  (params (OverlappedComponent :type "PrimitiveComponent Object Reference") (OtherActor :type "Actor Object Reference") (OtherComp :type "PrimitiveComponent Object Reference") (OtherBodyIndex :type Integer) (bFromSweep :type Boolean) (SweepResult :type "HitResult Structure (by ref)"))
  (if (!= OtherActor (`self.Instigator`))
    (`self.OnProjectileImpact` null)
    (`|ExecutionSequence`
      (:`then_0`
        (`self.ApplyDamage` OtherActor))
      (:`then_1`
        (`self.DestroyProjectile`)))))

(event `self.Sphere.OnComponentHit`
  (params (HitComponent :type "PrimitiveComponent Object Reference") (OtherActor :type "Actor Object Reference") (OtherComp :type "PrimitiveComponent Object Reference") (NormalImpulse :type "Vector Structure") (Hit :type "HitResult Structure (by ref)"))
  (`self.DestroyProjectile`))

(event `RotateToTarget`
  (bind _projectilemovement (`self.ProjectileMovement`))
  (set `MovementComponent.Velocity` (* (`KismetMathLibrary.GetDirectionUnitVector` (`self.K2_GetActorLocation`) (`self.K2_GetActorLocation` (`self.TargetActor`))) (`ProjectileMovementComponent.InitialSpeed` _projectilemovement)) _projectilemovement))

(event `DestroyProjectile`
  ; Destroy Projectile
  (`self.ReturnToPool`)
  ;;[0.3193 0 1 0.5] JUICE: Destroy cue
  (`GameplayCueFunctionLibrary.ExecuteGameplayCueOnActor` self (`self.ImpactGameplayCue`) (`AbilitySystemBlueprintLibrary.MakeGameplayCueParameters` 0.0 0.0 (struct) (struct) (struct) (struct) (struct) (`self.K2_GetActorLocation`))))

(event `FireProjectile`
  ;[0.3193 0 1 0.5] JUICE: Spawn cue
  (`GameplayCueFunctionLibrary.ExecuteGameplayCueOnActor` self (`self.SpawnGameplayCue`) (`AbilitySystemBlueprintLibrary.MakeGameplayCueParameters` 0.0 0.0 (struct) (struct) (struct) (struct) (struct) (`self.K2_GetActorLocation`)))
  (`self.TargetActor`
    (:`then`
      (if (`self.Homing?`)
        (set `ProjectileMovementComponent.HomingTargetComponent` (`Actor.RootComponent` (`self.TargetActor`)) (`self.ProjectileMovement`))
        (else
          (`self.RotateToTarget`))))
    (:`else`)))

(fn `ApplyDamage`
  (params (OtherActor :type "Actor Object Reference"))
  (bind _returnvalue (`AbilitySystemBlueprintLibrary.GetAbilitySystemComponent` OtherActor))
  ; GAS damage
  (`/Engine/EditorBlueprintResources/StandardMacros.IsValid` _returnvalue ; Does hit actor have ability system?
    (:`Is Valid`
      (`/Engine/EditorBlueprintResources/ActorMacros.Switch Has Authority`
        (:`Authority`
          (bind _returnvalue_2 (`AbilitySystemBlueprintLibrary.MakeSpecHandleByClass` "/Game/Game/Core/Blueprints/Combatants/Abilities/Effects/GE_DamageInstant.GE_DamageInstant_C"))
          (bind _returnvalue_3 (`AbilitySystemBlueprintLibrary.AssignTagSetByCallerMagnitude` _returnvalue_2 (struct :`TagName` "Data.Damage") (`self.Damage`)))
          (`AbilitySystemComponent.BP_ApplyGameplayEffectSpecToSelf` _returnvalue _returnvalue_3))))))

(fn `UserConstructionScript`
  (bind _projectilemovement (`self.ProjectileMovement`))
  (`parent.UserConstructionScript`)
  (set `ProjectileMovementComponent.InitialSpeed` (`self.Speed`) _projectilemovement)
  (set `ProjectileMovementComponent.MaxSpeed` (`self.MaxSpeed`) _projectilemovement))