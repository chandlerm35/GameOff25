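; BP_SuperWave is a projectile actor that shows a wave of three rings scaling in sequence.
; BeginPlay fills the Rings array and starts a looping 0.6-second timer that calls Fire.
; Fire steps an index, and each of the first three shots reveals one ring, scales it through its own Timeline, then hides it.
; The timer is never cleared, overlap handling is empty, and the destroy logic is unconnected.
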(event `self.ReceiveBeginPlay`
  (`self.PopulateRingArray`)
  (`self.Firing Sequence`))

(event `Firing Sequence`
  (bind _result (`/Engine/EditorBlueprintResources/StandardMacros.DecrementInt` (`KismetArrayLibrary.Array_Length` (`self.Rings`)))
    (:`  `
      (`KismetSystemLibrary.K2_SetTimerDelegate` (delegate `Fire`) 0.6 (>= _result (`self.MyIndex`)) true))))

(event `End`)

(event `self.Ring1.OnComponentBeginOverlap`
  (params (OverlappedComponent :type "PrimitiveComponent Object Reference") (OtherActor :type "Actor Object Reference") (OtherComp :type "PrimitiveComponent Object Reference") (OtherBodyIndex :type Integer) (bFromSweep :type Boolean) (SweepResult :type "HitResult Structure (by ref)")))

(event `Fire`
  (bind _ring2 (`self.Ring2`))
  (set `self.LocalIndex` (`self.MyIndex`))
  (`/Engine/EditorBlueprintResources/StandardMacros.IncrementInt` (`self.MyIndex`)
    (:`  `
      (switch `int` (`self.LocalIndex`)
        (:`0`
          (`SceneComponent.SetVisibility` (`self.Ring1`) true true)
          (bind (_direction _newtrack_0) (`Timeline|Timeline` :!via `PlayFromStart`)
            (:`Update`
              (`SceneComponent.SetRelativeScale3D` (`self.Ring1`) (`KismetMathLibrary.Conv_DoubleToVector` _newtrack_0)))
            (:`Finished`
              (`SceneComponent.SetVisibility` (`self.Ring1`) false true))))
        (:`1`
          (`SceneComponent.SetVisibility` _ring2 true true)
          (bind (_direction_2 _newtrack_0_2) (`Timeline|Timeline_2` :!via `PlayFromStart`)
            (:`Update`
              (`SceneComponent.SetRelativeScale3D` _ring2 (`KismetMathLibrary.Conv_DoubleToVector` _newtrack_0_2)))
            (:`Finished`
              (`SceneComponent.SetVisibility` _ring2 false true))))
        (:`2`
          (`SceneComponent.SetVisibility` (`self.Ring3`) true true)
          (bind (_direction_3 _newtrack_0_3) (`Timeline|Timeline_3` :!via `PlayFromStart`)
            (:`Update`
              (`SceneComponent.SetRelativeScale3D` (`self.Ring3`) (`KismetMathLibrary.Conv_DoubleToVector` _newtrack_0_3)))
            (:`Finished`
              (`SceneComponent.SetVisibility` (`self.Ring3`) false true))))))))

(event `FireNext`)

(fn `PopulateRingArray`
  (bind _rings (`self.Rings`))
  (`KismetArrayLibrary.Array_Add` _rings (`self.Ring1`))
  (`KismetArrayLibrary.Array_Add` _rings (`self.Ring2`))
  (`KismetArrayLibrary.Array_Add` _rings (`self.Ring3`))
  (for _ (`self.Rings`)
    _))

(fn `UserConstructionScript`)