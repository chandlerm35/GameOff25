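; Base projectile for an unblockable wave that launches toward a target location with a spawn gameplay cue.
; Box overlaps skip the instigator, BP_Shield actors and ignored classes, then apply server-only GAS damage through a SetByCaller effect to targets with an ability system.
; The wave passes through what it hits: shield-tag blocking, energy reward, destroy cue and return-to-pool logic exist but are disconnected.
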(event `self.ReceiveBeginPlay`)

(event `DestroyCue`
  ;[0.3193 0 1 0.5] JUICE: Destroy cue
  (`GameplayCueFunctionLibrary.ExecuteGameplayCueOnActor` self (`self.ImpactGameplayCue_0`) (`AbilitySystemBlueprintLibrary.MakeGameplayCueParameters` 0.0 0.0 (struct) (struct) (struct) (struct) (struct) (`self.K2_GetActorLocation`))))

(event `FireProjectile`
  (params (TargetLocation :type "Vector Structure"))
  (bind _projectilemovement (`self.ProjectileMovement`))
  ; Fire Projectile
  ;;[0.3193 0 1 0.5] JUICE: Spawn cue
  (`GameplayCueFunctionLibrary.ExecuteGameplayCueOnActor` self (`self.SpawnGameplayCue_0`) (`AbilitySystemBlueprintLibrary.MakeGameplayCueParameters` 0.0 0.0 (struct) (struct) (struct) (struct) (struct) (`self.K2_GetActorLocation`)))
  (set `self.TargetLocation` TargetLocation)
  (set `MovementComponent.Velocity` (* (`KismetMathLibrary.GetDirectionUnitVector` (`self.K2_GetActorLocation`) (`self.TargetLocation`)) (`self.Speed`)) _projectilemovement)
  (`ActorComponent.Activate` _projectilemovement false))

(event `self.Box.OnComponentBeginOverlap`
  (params (OverlappedComponent :type "PrimitiveComponent Object Reference") (OtherActor :type "Actor Object Reference") (OtherComp :type "PrimitiveComponent Object Reference") (OtherBodyIndex :type Integer) (bFromSweep :type Boolean) (SweepResult :type "HitResult Structure (by ref)"))
  ; Projectile Impact
  (if (!= OtherActor (`self.Instigator`))
    (if (not (`GameplayStatics.ObjectIsA` OtherActor "/Game/Game/Core/Blueprints/Actors/BP_Shield.BP_Shield_C"))
      (bind _ignoreactor_ (`self.ShouldActorBeIgnored?` OtherActor)) ; This should actually probably be done by collison channels
      (if (not _ignoreactor_)
        (`/Engine/EditorBlueprintResources/StandardMacros.IsValid` (`AbilitySystemBlueprintLibrary.GetAbilitySystemComponent` OtherActor)
          (:`Is Valid`
            ;; Maybe wave shouldnt be destroyed unless blocked
            (`self.ApplyDamage` OtherActor (`self.Instigator`)))
          (:`Is Not Valid`))))))

(event `self.Box.OnComponentHit`
  (params (HitComponent :type "PrimitiveComponent Object Reference") (OtherActor :type "Actor Object Reference") (OtherComp :type "PrimitiveComponent Object Reference") (NormalImpulse :type "Vector Structure") (Hit :type "HitResult Structure (by ref)"))
  ; Projectile Impact
)

(fn `ApplyDamage`
  (params (OtherActor :type "Actor Object Reference") (`Instigator Actor` :type "Actor Object Reference"))
  (bind _returnvalue (`AbilitySystemBlueprintLibrary.GetAbilitySystemComponent` OtherActor))
  ; GAS damage
  (`/Engine/EditorBlueprintResources/StandardMacros.IsValid` _returnvalue ; Does hit actor have ability system?
    (:`Is Valid`
      (`/Engine/EditorBlueprintResources/ActorMacros.Switch Has Authority`
        (:`Authority`
          (message `/Game/Game/Core/Blueprints/Data/Interface/BPI_Player.Fn_Set_Current_HitInstigator` (`local.OtherActor`) (`local.Instigator Actor`))
          (bind _returnvalue_2 (`AbilitySystemBlueprintLibrary.MakeSpecHandleByClass` "/Game/Game/Core/Blueprints/Combatants/Abilities/Effects/GE_DamageInstant.GE_DamageInstant_C"))
          (bind _returnvalue_3 (`AbilitySystemBlueprintLibrary.AssignTagSetByCallerMagnitude` _returnvalue_2 (struct :`TagName` "Data.Damage") (`self.Damage`)))
          (`AbilitySystemComponent.BP_ApplyGameplayEffectSpecToSelf` _returnvalue _returnvalue_3))))))

(fn `ApplyEnergy`
  (params (OtherActor :type "Actor Object Reference") (`Instigator Actor` :type "Actor Object Reference"))
  (bind _returnvalue (`AbilitySystemBlueprintLibrary.GetAbilitySystemComponent` OtherActor))
  ; GAS damage
  (`/Engine/EditorBlueprintResources/StandardMacros.IsValid` _returnvalue ; Does hit actor have ability system?
    (:`Is Valid`
      (`/Engine/EditorBlueprintResources/ActorMacros.Switch Has Authority`
        (:`Authority`
          (message `/Game/Game/Core/Blueprints/Data/Interface/BPI_Player.Fn_Set_Current_HitInstigator` (`local.OtherActor`) (`local.Instigator Actor`))
          (bind _returnvalue_2 (`AbilitySystemBlueprintLibrary.MakeSpecHandleByClass` "/Game/Game/Core/Blueprints/Combatants/Abilities/Effects/GE_ChangeEnergy.GE_ChangeEnergy_C"))
          (bind _returnvalue_3 (`AbilitySystemBlueprintLibrary.AssignTagSetByCallerMagnitude` _returnvalue_2 (struct :`TagName` "Data.Energy") (`self.EnergyGivenWhenBlocked`)))
          (`AbilitySystemComponent.BP_ApplyGameplayEffectSpecToSelf` _returnvalue _returnvalue_3))))))

(fn `ShouldActorBeIgnored?`
  (params (ActorToTest :type "Actor Object Reference"))
  (returns (`IgnoreActor?` :type Boolean))
  (locals (LocalSuccess :type Boolean))
  (bind _classestoignore (`self.ClassesToIgnore`))
  (set `local.LocalSuccess` false)
  (if (> (`KismetArrayLibrary.Array_Length` _classestoignore) 0)
    (for _array_element _classestoignore
      (if (`GameplayStatics.ObjectIsA` ActorToTest _array_element)
        (set `local.LocalSuccess` true)
        (break)))
    (return (`local.LocalSuccess`))))

(fn `UserConstructionScript`)