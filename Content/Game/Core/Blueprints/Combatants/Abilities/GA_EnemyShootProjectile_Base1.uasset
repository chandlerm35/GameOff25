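; Base gameplay ability for enemy projectile shooting; as wired, activation only commits the ability and never fires or ends it.
; A disconnected chain line-traces toward the forward vector scaled as a world position, pulls ProjectileClass from the avatar's AC_MultiObjectPool, fires it at the impact point, then ends the ability.
; That unreachable chain prints an error when the pool component is invalid.
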(event `self.K2_ActivateAbility`
  (`self.K2_CommitAbility`))