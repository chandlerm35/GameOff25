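; Gameplay ability for the boss's super wave attack, telegraphed by a spawned-text countdown from Four to One.
; After the countdown, a looping timer spawns partial superwave projectiles carrying the ability's damage, aimed by a forward line trace, with a firing sound.
; The ability clears the timer and ends once the wave count is reached.
; Its end handler casts the avatar to the player character before removing the granted ability.
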(event `self.K2_ActivateAbility`
  (bind _asbp_boss (cast `/Game/Game/Core/Blueprints/Combatants/Enemy/BP_Boss` (`self.GetAvatarActorFromActorInfo`)))
  (`/Game/Game/Core/Blueprints/Combatants/Enemy/BP_BossBase.BossSpecial` _asbp_boss)
  (`/Game/Game/Core/Blueprints/Combatants/BP_CombatantBase.Fn_BonusTextSpawn_Call` _asbp_boss "Four")
  (`KismetSystemLibrary.Delay` 1.0)
  (`/Game/Game/Core/Blueprints/Combatants/BP_CombatantBase.Fn_BonusTextSpawn_Call` _asbp_boss "Three")
  (`KismetSystemLibrary.Delay` 1.0)
  (`/Game/Game/Core/Blueprints/Combatants/BP_CombatantBase.Fn_BonusTextSpawn_Call` _asbp_boss "Two")
  (`KismetSystemLibrary.Delay` 1.0)
  (`/Game/Game/Core/Blueprints/Combatants/BP_CombatantBase.Fn_BonusTextSpawn_Call` _asbp_boss "One")
  (`KismetSystemLibrary.Delay` 1.0)
  (bind _returnvalue (`KismetSystemLibrary.K2_SetTimerDelegate` (`|CreateDelegate` :!event `Fire`) 0.6 true true))
  (set `self.Timer` _returnvalue))

(event `Fire`
  (bind _returnvalue (`self.GetAvatarActorFromActorInfo`))
  (bind _returnvalue_2 (`self.GetAvatarActorFromActorInfo`))
  (bind _returnvalue_3 (`|SpawnActorFromClass` "/Game/Game/Core/Blueprints/Actors/Projectiles/BP_PartialSuperwave.BP_PartialSuperwave_C" (`Actor.GetTransform` _returnvalue_2) "Undefined" "MultiplyWithRoot" _returnvalue_2 1000.0 (0.0 0.0 0.0) (struct) (cast `Pawn` _returnvalue_2 :!pure true)))
  (set `/Game/Game/Core/Blueprints/Actors/Projectiles/BP_UnblockableWaveBase.Damage` (`self.AbilityDamage`) _returnvalue_3)
  (bind _outhit (`KismetSystemLibrary.LineTraceSingle` (`Actor.K2_GetActorLocation` _returnvalue) (* (`Actor.GetActorForwardVector` _returnvalue) 100000.0) "TraceTypeQuery1"))
  (`/Game/Game/Core/Blueprints/Actors/Projectiles/BP_UnblockableWaveBase.FireProjectile` _returnvalue_3 (`.ImpactPoint` (`GameplayStatics.BreakHitResult` _outhit)))
  ;[0.3193 0 1 0.5] SFX
  (`FMODBlueprintStatics.PlayEventAtLocation` "/Game/FMOD/Events/GameSFX/SuperWaveFire.SuperWaveFire" (`KismetMathLibrary.Conv_VectorToTransform` (`Actor.K2_GetActorLocation` (`self.GetAvatarActorFromActorInfo`))))
  (`/Engine/EditorBlueprintResources/StandardMacros.IncrementInt` (`self.MyIndex`)
    (:`  `
      (if (not (>= (- (`self.WavesToFire`) 1) (`self.MyIndex`)))
        (`KismetSystemLibrary.K2_ClearAndInvalidateTimerHandle` (`self.Timer`))
        (`self.K2_EndAbility`)))))

(event `self.K2_OnEndAbility`
  (params (bWasCancelled :type Boolean))
  (bind _returnvalue (`self.GetAvatarActorFromActorInfo`))
  (bind _asbp_player_character (cast `/Game/Game/Core/Blueprints/Combatants/Player/BP_PlayerCharacter` _returnvalue))
  (`AbilitySystemComponent.ClearAbility` (`AbilitySystemBlueprintLibrary.GetAbilitySystemComponent` _returnvalue) (`/Game/Game/Core/Blueprints/Combatants/Player/BP_PlayerCharacter.SuperWaveHandle` _asbp_player_character)))