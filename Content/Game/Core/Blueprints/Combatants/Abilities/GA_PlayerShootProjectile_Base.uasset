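; Base gameplay ability for player projectile shooting, firing a pooled projectile from the avatar's location.
; On activation it commits, then line-traces along the avatar's forward vector to get an impact point.
; The avatar's AC_MultiObjectPool spawns the configured ProjectileClass, which fires toward that point, whether or not the trace hit.
; The ability ends only after a successful shot; a missing pool just prints an error.
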(event `self.K2_ActivateAbility`
  (bind _returnvalue (`self.GetAvatarActorFromActorInfo`))
  (bind _returnvalue_2 (`self.GetAvatarActorFromActorInfo`))
  (bind _output (`|GetArrayItem` (`Actor.K2_GetComponentsByClass` _returnvalue "/Game/Game/Core/Blueprints/Components/AC_MultiObjectPool.AC_MultiObjectPool_C")))
  (`self.K2_CommitAbility`)
  (bind _outhit (`KismetSystemLibrary.LineTraceSingle` (`Actor.K2_GetActorLocation` _returnvalue_2) (* (`Actor.GetActorForwardVector` _returnvalue_2) 100000.0) "TraceTypeQuery1"))
  (`/Engine/EditorBlueprintResources/StandardMacros.IsValid` _output
    (:`Is Valid`
      (bind _pooledactor (`/Game/Game/Core/Blueprints/Components/AC_MultiObjectPool.SpawnFromPool` _output (`KismetMathLibrary.MakeTransform` (`Actor.K2_GetActorLocation` (`self.GetAvatarActorFromActorInfo`))) (`self.ProjectileClass`)))
      (bind _asbp_base_projectile (cast `/Game/Game/Core/Blueprints/Actors/Projectiles/BP_BaseProjectile` _pooledactor))
      (`/Game/Game/Core/Blueprints/Actors/Projectiles/BP_BaseProjectile.FireProjectile` _asbp_base_projectile (`.ImpactPoint` (`GameplayStatics.BreakHitResult` _outhit)))
      (`self.K2_EndAbility`))
    (:`Is Not Valid`
      (`KismetSystemLibrary.PrintString` (`KismetTextLibrary.Conv_TextToString` (`|FormatText` "MultiPool component is not valid on {Actor} when trying to use ability {ability}" _returnvalue self)) true true (struct :`R` 1.0 :`G` 0.00584 :`A` 1.0) 30.0))))