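; GA_PlayerSuperWave is a one-shot gameplay ability for the player's super wave attack.
; On activation it commits the cost, spawns BP_SuperWave at the avatar's transform with the avatar as owner and instigator, adds a gameplay cue and ends immediately.
; On end it clears itself from the ability system component using the SuperWaveHandle stored on BP_PlayerCharacter, so each use requires a new grant.
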(event `self.K2_ActivateAbility`
  (bind _returnvalue (`self.GetAvatarActorFromActorInfo`))
  (`KismetSystemLibrary.PrintString` "ActivateSuperWave" true true (struct :`G` 0.66 :`B` 1.0 :`A` 1.0) 2.0 "None")
  (`self.K2_CommitAbilityCost` false)
  (`|SpawnActorFromClass` "/Game/Game/Core/Blueprints/Actors/Projectiles/BP_SuperWave.BP_SuperWave_C" (`Actor.GetTransform` _returnvalue) "Undefined" "MultiplyWithRoot" _returnvalue (cast `Pawn` _returnvalue :!pure true))
  (`self.K2_AddGameplayCue` (struct))
  (`self.K2_EndAbility`))

(event `self.K2_OnEndAbility`
  (params (bWasCancelled :type Boolean))
  (bind _returnvalue (`self.GetAvatarActorFromActorInfo`))
  (bind _asbp_player_character (cast `/Game/Game/Core/Blueprints/Combatants/Player/BP_PlayerCharacter` _returnvalue))
  (`AbilitySystemComponent.ClearAbility` (`AbilitySystemBlueprintLibrary.GetAbilitySystemComponent` _returnvalue) (`/Game/Game/Core/Blueprints/Combatants/Player/BP_PlayerCharacter.SuperWaveHandle` _asbp_player_character)))