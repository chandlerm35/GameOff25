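; GA_ShieldBase is a base Gameplay Ability that raises a shield around the avatar actor.
; On activation it commits the cooldown, spawns a BP_Shield owned by the avatar, and plays the ShieldUp sound event at the avatar's location.
; It applies the ShieldMaterial variable, attaches the shield to the avatar and activates it.
; When the ability ends, it deactivates the shield if still valid.
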(event `self.K2_ActivateAbility`
  (bind _returnvalue (`self.GetAvatarActorFromActorInfo`))
  (bind _shield (`self.Shield`))
  (`self.K2_CommitAbilityCooldown` false)
  (bind _returnvalue_2 (`|SpawnActorFromClass` "/Game/Game/Core/Blueprints/Actors/BP_Shield.BP_Shield_C" (`KismetMathLibrary.MakeTransform` (0.0 0.0 0.0)) "Undefined" "MultiplyWithRoot" _returnvalue (cast `Pawn` _returnvalue :!pure true)))
  (`FMODBlueprintStatics.PlayEventAtLocation` "/Game/FMOD/Events/GameSFX/ShieldUp.ShieldUp" (`KismetMathLibrary.Conv_VectorToTransform` (`Actor.K2_GetActorLocation` (`self.GetAvatarActorFromActorInfo`))))
  (bind _output_get (set `self.Shield` _returnvalue_2))
  (`/Game/Game/Core/Blueprints/Actors/BP_Shield.SetMaterial` _shield (`self.ShieldMaterial`))
  (`/Game/Game/Core/Blueprints/Actors/BP_Shield.SetMaterial` _output_get (`self.ShieldMaterial`))
  (`Actor.K2_AttachToActor` _shield (`self.GetAvatarActorFromActorInfo`) "None" "SnapToTarget" "KeepRelative" "KeepRelative" false)
  (`/Game/Game/Core/Blueprints/Actors/BP_Shield.Activate` (`self.Shield`)))

(event `self.K2_OnEndAbility`
  (params (bWasCancelled :type Boolean))
  (bind _shield (`self.Shield`)
    (:`then`
      (`/Game/Game/Core/Blueprints/Actors/BP_Shield.Deactivate` _shield))
    (:`else`)))