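; Gameplay Ability that shoots a projectile by spawning it from the avatar actor's AC_ObjectPool component at the avatar's transform.
; With a valid pool, activation commits the cooldown, spawns and ends; otherwise it prints an error without ending the ability.
; AddProjectilePool, not called in this graph, adds a pool component to the avatar for the Projectile class.
; The SetByCaller damage effect spec logic is disconnected and never runs.
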(event `self.K2_ActivateAbility`
  (bind _returnvalue (`self.GetAvatarActorFromActorInfo`))
  (bind _returnvalue_2 (`Actor.GetComponentByClass` _returnvalue "/Game/Game/Core/Blueprints/Components/AC_ObjectPool.AC_ObjectPool_C"))
  (bind _result (`|FormatText` "{Component} on {Actor} is invalid while trying to activate {Ability}" _returnvalue_2 _returnvalue self))
  (`/Engine/EditorBlueprintResources/StandardMacros.IsValid` _returnvalue_2
    (:`Is Valid`
      (`self.K2_CommitAbilityCooldown` false)
      (`/Game/Game/Core/Blueprints/Components/AC_ObjectPool.SpawnFromPool` _returnvalue_2 (`Actor.GetTransform` _returnvalue))
      (`self.K2_EndAbility`))
    (:`Is Not Valid`
      (`KismetSystemLibrary.PrintString` (`KismetTextLibrary.Conv_TextToString` _result) true true (struct :`R` 1.0 :`B` 0.208135 :`A` 1.0) 30.0 (`KismetStringLibrary.Conv_StringToName` (`KismetTextLibrary.Conv_TextToString` _result))))))

(fn `AddProjectilePool`
  (bind _returnvalue (`|AddComponentByClass` (`self.GetAvatarActorFromActorInfo`) "/Game/Game/Core/Blueprints/Components/AC_ObjectPool.AC_ObjectPool_C" (`self.Projectile`)))
  (set `/Game/Game/Core/Blueprints/Components/AC_ObjectPool.PooledActorClass` (`self.Projectile`) _returnvalue))