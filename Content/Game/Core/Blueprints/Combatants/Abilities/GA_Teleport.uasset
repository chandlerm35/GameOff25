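; Gameplay ability that performs the teleport as a short, fast root-motion burst in the pawn's last movement input direction, or actor forward without input.
; Activation commits cost, applies a constant-force root motion task and adds a gameplay cue removed on ability end.
; On finish, it commits cooldown and ends.
; Exit velocity is clamped to the movement component's max speed, with a fallback value for non-pawn avatars.
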(event `self.K2_ActivateAbility`
  (`self.K2_CommitAbilityCost` false)
  (`AbilityTask_ApplyRootMotionConstantForce.ApplyRootMotionConstantForce` "None" (`self.GetDirection`) 2400.0 0.2 false null "ClampVelocity" (0.0 0.0 0.0) (`self.GetMaxMoveSpeed`)
    (:`then`
      (`self.K2_AddGameplayCue` (struct)))
    (:`OnFinish`
      (`self.K2_CommitAbilityCooldown` false)
      (`self.K2_EndAbility`))))

(fn `GetDirection`
  (returns (Vector :type "Vector Structure"))
  (bind _aspawn (cast `Pawn` (`self.GetAvatarActorFromActorInfo`))
    (:`then`
      (bind _returnvalue (`Pawn.GetLastMovementInputVector` _aspawn))
      (if (`KismetMathLibrary.Vector_IsZero` _returnvalue)
        _
        (else
          (return _returnvalue))))
    (:`CastFailed`
      _))
  (return (`Actor.GetActorForwardVector` (`self.GetAvatarActorFromActorInfo`))))

(fn `GetMaxMoveSpeed`
  (returns (ReturnValue :type "Float (single-precision)"))
  (bind _aspawn (cast `Pawn` (`self.GetAvatarActorFromActorInfo`))
    (:`then`
      (return (`MovementComponent.GetMaxSpeed` (`Pawn.GetMovementComponent` _aspawn))))
    (:`CastFailed`
      (return (`self.FallbackEndVelocity`)))))