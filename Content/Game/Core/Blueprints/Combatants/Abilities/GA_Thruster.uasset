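; Thruster gameplay ability that gives the avatar character a temporary speed boost.
; On activation it commits the cooldown (noted as UI-only), adds VelocityBoost to MaxWalkSpeed and plays the Thruster movement gameplay cue.
; After DashDuration it restores the saved speed and ends, which also removes the cue.
; Helpers for querying max speed and spawning velocity-driven charging dust are defined but not called in the event graph.
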(event `self.K2_ActivateAbility`
  ;[0.15 0.15 0.15 0.5 14] Just for UI, no gameplay impact
  (`self.K2_CommitAbilityCooldown` false)
  (bind _ascharacter (cast `Character` (`self.GetAvatarActorFromActorInfo`)))
  (bind _charactermovement (`Character.CharacterMovement` _ascharacter))
  (bind _maxwalkspeed (`CharacterMovementComponent.MaxWalkSpeed` _charactermovement))
  (set `self.StartMaxMoveSpeed` _maxwalkspeed)
  (set `CharacterMovementComponent.MaxWalkSpeed` (+ _maxwalkspeed (`self.VelocityBoost`)) _charactermovement)
  (`self.K2_AddGameplayCue` (struct :`TagName` "GameplayCue.Movement.Thruster"))
  (`KismetSystemLibrary.Delay` (`self.DashDuration`))
  (set `CharacterMovementComponent.MaxWalkSpeed` (`self.StartMaxMoveSpeed`) _charactermovement)
  (`self.K2_EndAbility`))

(fn `GetMaxMoveSpeed`
  (returns (ReturnValue :type "Float (single-precision)"))
  (bind _aspawn (cast `Pawn` (`self.GetAvatarActorFromActorInfo`))
    (:`then`
      (return (`MovementComponent.GetMaxSpeed` (`Pawn.GetMovementComponent` _aspawn))))
    (:`CastFailed`
      (return 0.0))))

(fn `Spawn Niagara FX`
  (bind _returnvalue (`self.GetAvatarActorFromActorInfo`))
  (bind _niagara_system_taken (message `/Game/Game/Core/Blueprints/Data/Interface/BPI_Player.Fn_GetNiagaraSystem_Attached` (`self.GetAvatarActorFromActorInfo`)))
  (bind _returnvalue_2 (`NiagaraFunctionLibrary.SpawnSystemAttached` "/Game/Game/Assets/Particles/NS_ChargingDust.NS_ChargingDust" _niagara_system_taken "None" (0.0 0.0 0.0) (struct) "KeepRelativeOffset" true true "AutoRelease"))
  (`NiagaraComponent.SetVariableVec3` _returnvalue_2 "DashDirection" (`Actor.GetVelocity` _returnvalue))
  (`NiagaraFunctionLibrary.OverrideSystemUserVariableSkeletalMeshComponent` _returnvalue_2 "CharacterMesh" (`Actor.GetComponentByClass` _returnvalue "/Script/Engine.SkeletalMeshComponent")))