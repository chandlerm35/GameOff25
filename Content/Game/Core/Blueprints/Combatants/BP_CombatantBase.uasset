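; BP_CombatantBase is a base combatant actor that gives hit feedback when it loses health.
; After a one-tick delay on BeginPlay, it initializes the damage FX component and keeps listening for attribute changes on itself.
; A decrease triggers a damage flash and a brief hit pause through the hit-apply component.
; Getter functions expose the controller and hit-apply component, while the widget component getter returns nothing.
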(event `self.ReceiveBeginPlay`
  (`KismetSystemLibrary.DelayUntilNextTick`)
  (`/Game/Game/Core/Blueprints/Components/AC_DamageFX.Initialize Hit Flash` (`self.AC_DamageFX`))
  (`/Engine/EditorBlueprintResources/StandardMacros.IsValid` self
    (:`Is Valid`
      (bind (_asynctaskproxy _attribute _newvalue _oldvalue) (`AbilityAsync_WaitAttributeChanged.WaitForAttributeChanged` self (struct :`AttributeName` "Health" :`Attribute` "/Script/GameOff25.BasicAttributeSet:Health" :`AttributeOwner` "/Script/CoreUObject.Class'/Script/GameOff25.BasicAttributeSet'"))
        (:`Changed`
          (if (not (== _newvalue _oldvalue))
            (`self.CallHitFlash` (< _newvalue _oldvalue))))))))

(fn `CallHitFlash`
  (params (`Is Losing Health?` :type Boolean))
  (if `Is Losing Health?`
    (`/Game/Game/Core/Blueprints/Components/AC_DamageFX.DamageFlash` (`self.AC_DamageFX`) self 0.0 null null null)
    (`/Game/Game/Core/Blueprints/Components/AC_Player_HitApply.Call Hit Pause` (`self.AC_Player_HitApply`) null "/Script/Engine.DamageType" 0.08)))

(fn `Fn_GetController`
  (returns (`Controller Attached` :type "Controller Object Reference"))
  (return (`self.GetController`)))

(fn `Fn_GetHitApply_AC`
  (returns (`Hit Apply AC` :type "/Game/Game/Core/Blueprints/Components/AC_Player_HitApply Object Reference"))
  (return (`self.AC_Player_HitApply`)))

(fn `Fn_GetWidgetComponent`
  (returns (`Widget Component` :type "WidgetComponent Object Reference"))
  (return null))

(fn `UserConstructionScript`)