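; BP_Boss is a boss enemy that fires two wave attacks through the Gameplay Ability System.
; On BeginPlay it waits for Wave1 and Wave2 gameplay events, activating the matching GA_ShootWave ability for each.
; BossSpecial replaces the StateTree component at runtime with a newly added one, which is replaced again when it succeeds.
; TestWave alternates both waves, but its looping timer is disconnected.
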(event `TestWave`
  (bind _abilitysystemcomponent (`self.AbilitySystemComponent`))
  (`/Engine/EditorBlueprintResources/StandardMacros.FlipFlop`
    (:`A`
      (`AbilitySystemComponent.TryActivateAbilityByClass` _abilitysystemcomponent "/Game/Game/Core/Blueprints/Combatants/Abilities/GA_ShootWave1.GA_ShootWave1_C" true))
    (:`B`
      (`AbilitySystemComponent.TryActivateAbilityByClass` _abilitysystemcomponent "/Game/Game/Core/Blueprints/Combatants/Abilities/GA_ShootWave2.GA_ShootWave2_C" true))))

(event `self.ReceiveBeginPlay`
  (`parent.ReceiveBeginPlay`)
  (`AbilityAsync_WaitGameplayEvent.WaitGameplayEventToActor` null (struct :`TagName` "Event.ActivateAbility.Wave1")
    (:`then`
      (`AbilityAsync_WaitGameplayEvent.WaitGameplayEventToActor` null (struct :`TagName` "Event.ActivateAbility.Wave2")
        (:`EventReceived`
          (`AbilitySystemComponent.TryActivateAbilityByClass` (`self.AbilitySystemComponent`) "/Game/Game/Core/Blueprints/Combatants/Abilities/GA_ShootWave2.GA_ShootWave2_C" true))))
    (:`EventReceived`
      (`AbilitySystemComponent.TryActivateAbilityByClass` (`self.AbilitySystemComponent`) "/Game/Game/Core/Blueprints/Combatants/Abilities/GA_ShootWave1.GA_ShootWave1_C" true))))

(event `self.BossSpecial`
  (bind _statetree (`self.StateTree`))
  (`BrainComponent.StopLogic` _statetree "Special Action")
  (`ActorComponent.K2_DestroyComponent` _statetree)
  (bind _returnvalue (`AddComponent|NODE_AddStateTreeComponent-0`))
  (set `self.StateTree` _returnvalue)
  (add `StateTreeComponent.OnStateTreeRunStatusChanged` _returnvalue (delegate `TreeFinished`)))

(event `TreeFinished`
  (params (StateTreeRunStatus :type "EStateTreeRunStatus Enum" :default "Running"))
  (switch `EStateTreeRunStatus` StateTreeRunStatus
    (:`Succeeded`
      (`BrainComponent.StopLogic` (`self.StateTree`) "Special Action Finished")
      (`ActorComponent.K2_DestroyComponent` (`self.StateTree`))
      (bind _returnvalue (`AddComponent|NODE_AddStateTreeComponent-1`))
      (set `self.StateTree` _returnvalue))))

(fn `UserConstructionScript`
  (`parent.UserConstructionScript`))