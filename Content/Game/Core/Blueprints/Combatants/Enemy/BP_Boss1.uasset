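; BP_Boss1 is an enemy boss combatant built on the Gameplay Ability System, still carrying test scaffolding.
; On BeginPlay it initializes BasicAttributeSet, creates a boss health bar widget and grants its KnownAbilities.
; An attribute-change listener reports health and calls OnDeath at zero, while a looping timer repeatedly activates GA_BossAttack1 as a test.
; An unused damage test applies a set-by-caller damage-over-time effect to itself.
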(event `DamageTest`
  ; TESTING HEALTH
  (bind _returnvalue (`AbilitySystemBlueprintLibrary.MakeSpecHandleByClass` "/Game/Game/Core/Blueprints/Combatants/Abilities/Effects/GE_DoT_Infinite.GE_DoT_Infinite_C" null self))
  (bind _returnvalue_2 (`AbilitySystemBlueprintLibrary.AssignTagSetByCallerMagnitude` _returnvalue (struct :`TagName` "Data.Damage") -25.0))
  (`AbilitySystemComponent.BP_ApplyGameplayEffectSpecToSelf` (`self.AbilitySystemComponent`) _returnvalue_2))

(event `self.ReceiveBeginPlay`
  (`parent.ReceiveBeginPlay`)
  (`self.Initialize`)
  (bind (_asynctaskproxy _attribute _newvalue) (`AbilityAsync_WaitAttributeChanged.WaitForAttributeChanged` null (struct :`AttributeName` "Health" :`Attribute` "/Script/GameOff25.BasicAttributeSet:Health" :`AttributeOwner` "/Script/CoreUObject.Class'/Script/GameOff25.BasicAttributeSet'")) ; This node can't be in a function
    (:`then`
      (`KismetSystemLibrary.K2_SetTimerDelegate` (delegate `AbilityTest`) 1.0 true))
    (:`Changed`
      (`self.HandleHealthChanged` _newvalue))))

(event `HandleHealthChanged`
  (params (Health :type "Float (double-precision)"))
  ; Health Changed
  (if (<= Health 0.0)
    (`self.OnDeath`)
    (`KismetSystemLibrary.PrintString` "Boss 1 called on death event" true true (struct :`G` 0.66 :`B` 1.0 :`A` 1.0) 30.0 "Boss1 has died")
    (else
      (`KismetSystemLibrary.PrintString` (`KismetTextLibrary.Conv_TextToString` (`|FormatText` "{actor} is at {health} health" (`KismetSystemLibrary.GetDisplayName` self) Health)) true true (struct :`R` 0.012736 :`G` 1.0 :`A` 1.0) 10.0 "BossHealthTest"))))

(event `AbilityTest`
  (`AbilitySystemComponent.TryActivateAbilityByClass` (`self.AbilitySystemComponent`) "/Game/Game/Core/Blueprints/Combatants/Abilities/GA_BossAttack1.GA_BossAttack1_C" true))

(fn `GiveAbilities`
  (for _array_element (`self.KnownAbilities`)
    (`AbilitySystemComponent.K2_GiveAbility` (`self.AbilitySystemComponent`) _array_element 0 -1)))

(fn `Initialize`
  (`AbilitySystemComponent.K2_InitStats` (`self.AbilitySystemComponent`) "/Script/GameOff25.BasicAttributeSet" null)
  (`self.AttributesInitialized`)
  ; Create health bar
  (`|CreateWidget` "/Game/Game/Core/UI/Widgets/WBP_BossHealthBar.WBP_BossHealthBar_C" null self)
  (`self.GiveAbilities`))

(fn `UserConstructionScript`
  (`parent.UserConstructionScript`))