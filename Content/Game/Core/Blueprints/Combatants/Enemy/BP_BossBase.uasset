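; BP_BossBase is a base boss enemy Blueprint built on the Gameplay Ability System, with temporary test hooks.
; On BeginPlay it initializes, listens for attribute changes as health, and waits for a shoot gameplay event to activate the base enemy projectile ability.
; Health at zero triggers death and notifies the game state; otherwise it prints debug health.
; Targeting temporarily uses the player pawn, and damage and timed-ability tests are disconnected.
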(event `DamageTest`
  ; TESTING HEALTH
  (bind _returnvalue (`AbilitySystemBlueprintLibrary.MakeSpecHandleByClass` "/Game/Game/Core/Blueprints/Combatants/Abilities/Effects/GE_DoT_Infinite.GE_DoT_Infinite_C" null self))
  (bind _returnvalue_2 (`AbilitySystemBlueprintLibrary.AssignTagSetByCallerMagnitude` _returnvalue (struct :`TagName` "Data.Damage") -25.0))
  (`AbilitySystemComponent.BP_ApplyGameplayEffectSpecToSelf` (`self.AbilitySystemComponent`) _returnvalue_2))

(event `self.ReceiveBeginPlay`
  (`self.Initialize`)
  (bind (_asynctaskproxy _attribute _newvalue) (`AbilityAsync_WaitAttributeChanged.WaitForAttributeChanged` null (struct :`AttributeName` "Health" :`Attribute` "/Script/GameOff25.BasicAttributeSet:Health" :`AttributeOwner` "/Script/CoreUObject.Class'/Script/GameOff25.BasicAttributeSet'")) ; This node can't be in a function
    (:`then`
      (`AbilityAsync_WaitGameplayEvent.WaitGameplayEventToActor` null (struct :`TagName` "Event.ActivateAbility.Shoot")
        (:`then`
          (`self.SetTargetActor`))
        (:`EventReceived`
          ; This may need a cooldown, or it only tries when ability is off cooldown
          (`AbilitySystemComponent.TryActivateAbilityByClass` (`self.AbilitySystemComponent`) "/Game/Game/Core/Blueprints/Combatants/Abilities/GA_EnemyShootProjectile_Base.GA_EnemyShootProjectile_Base_C" true :!label _label))))
    (:`Changed`
      (`self.HandleHealthChanged` _newvalue))))

(event `HandleHealthChanged`
  (params (Health :type "Float (double-precision)"))
  ; Health Changed
  (if (<= Health 0.0)
    (`self.OnDeath` null)
    (`/Game/Game/Core/Blueprints/GameModes/GS_GameState_Game.BossDeath` (`self.Gamestate`))
    (else
      (`KismetSystemLibrary.PrintString` (`KismetTextLibrary.Conv_TextToString` (`|FormatText` "{actor} is at {health} health" (`KismetSystemLibrary.GetDisplayName` self) Health)) true true (struct :`R` 0.012736 :`G` 1.0 :`A` 1.0) 10.0 "BossHealthTest"))))

(event `AbilityTest`
  ; This may need a cooldown, or it only tries when ability is off cooldown
  (goto _label))

(event `SetTargetActor`
  ; Get target actor
  (set `self.TargetActor` (`GameplayStatics.GetPlayerPawn` 0)))

(fn `UserConstructionScript`
  (`parent.UserConstructionScript`))