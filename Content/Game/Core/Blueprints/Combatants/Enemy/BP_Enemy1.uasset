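; BP_Enemy1 is an enemy combatant Blueprint that shoots projectiles and shows a sprite look matched to its AI class.
; On BeginPlay it listens for the Event.ActivateAbility.Shoot gameplay event and activates GA_EnemyShootProjectile_Base through its Ability System Component.
; When its AI is set, it looks up a sprite material for that AI in ClassSpriteMaterials, falling back to M_EnemySprite.
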(event `self.ReceiveBeginPlay`
  (`parent.ReceiveBeginPlay`)
  (`AbilityAsync_WaitGameplayEvent.WaitGameplayEventToActor` null (struct :`TagName` "Event.ActivateAbility.Shoot")
    (:`EventReceived`
      (`AbilitySystemComponent.TryActivateAbilityByClass` (`self.AbilitySystemComponent`) "/Game/Game/Core/Blueprints/Combatants/Abilities/GA_EnemyShootProjectile_Base.GA_EnemyShootProjectile_Base_C" true))))

(event `self.SetAI`
  (params (NewAI :type Name))
  (bind _papersprite (`self.PaperSprite`))
  (bind (_value _returnvalue) (`BlueprintMapLibrary.Map_Find` (`self.ClassSpriteMaterials`) NewAI))
  (`parent.SetAI` NewAI)
  (if _returnvalue
    (`PrimitiveComponent.SetMaterial` _papersprite 0 _value)
    (else
      (`PrimitiveComponent.SetMaterial` _papersprite 0 "/Game/Game/Assets/Materials/Enemies/M_EnemySprite.M_EnemySprite"))))

(fn `UserConstructionScript`
  (`parent.UserConstructionScript`))