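; Base enemy actor built for pooling, with GAS-driven health, abilities, an on-field health bar and a StateTree.
; BeginPlay hides it, initializes attributes, grants abilities and temporarily targets the player pawn.
; SetInUse toggles collision, visibility and tick, and on activation resets health and starts the StateTree.
; Zero health broadcasts OnDeath, plays an explosion sound, deactivates components and adds a RoboticDeath component, which ReturnToPool destroys.
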(event `self.ReceiveBeginPlay`
  (`parent.ReceiveBeginPlay`)
  (`self.SetInUse` false)
  (`self.Initialize`)
  (bind (_asynctaskproxy _attribute _newvalue) (`AbilityAsync_WaitAttributeChanged.WaitForAttributeChanged` null (struct :`AttributeName` "Health" :`Attribute` "/Script/GameOff25.BasicAttributeSet:Health" :`AttributeOwner` "/Script/CoreUObject.Class'/Script/GameOff25.BasicAttributeSet'")) ; This node can't be in a function
    (:`then`
      (`self.SetTargetActor`))
    (:`Changed`
      (`self.HandleHealthChanged` _newvalue))))

(event `SetTargetActor`
  ; Get target actor
  (set `self.TargetActor` (`GameplayStatics.GetPlayerPawn` 0)))

(event `HandleHealthChanged`
  (params (Health :type "Float (double-precision)"))
  ; Health Changed
  (if (<= Health 0.0)
    (`self.OnDeath` self)
    ;;[0.3193 0 1 0.5] SFX
    (`FMODBlueprintStatics.PlayEventAtLocation` "/Game/FMOD/Events/GameSFX/Explosions/MiniExplosion.MiniExplosion" (`KismetMathLibrary.MakeTransform` (`self.K2_GetActorLocation`)))
    ;; Remove components and explode
    (`self.SetActorEnableCollision` false)
    (`KismetSystemLibrary.DelayUntilNextTick`)
    (`ActorComponent.Deactivate` (`self.AC_Player_HitApply`))
    (`ActorComponent.Deactivate` (`self.StateTree`))
    (`ActorComponent.Deactivate` (`self.AC_DamageFX`))
    (`ActorComponent.Deactivate` (`self.UIA_OnFieldDisplayHUD`))
    (`ActorComponent.Deactivate` (`self.AbilitySystemComponent`))
    (bind _returnvalue (`AddComponent|NODE_AddAC_RoboticDeath-0`))
    (set `self.RoboticDeath` _returnvalue)))

(event `SetInUse`
  (params (InUse :type Boolean))
  ; Pooled function, set in use
  (set `self.InUse` InUse)
  (`self.SetActorEnableCollision` InUse)
  (`self.SetActorHiddenInGame` (not InUse))
  (`self.SetActorTickEnabled` InUse)
  (if InUse
    (`ActorComponent.Activate` (`self.StateTree`) false)
    (`ActorComponent.Activate` (`self.AC_DamageFX`) false)
    (`ActorComponent.Activate` (`self.AC_Player_HitApply`) false)
    (`ActorComponent.Activate` (`self.UIA_OnFieldDisplayHUD`) false)
    (`ActorComponent.Activate` (`self.AbilitySystemComponent`) false)
    (`self.ResetHealth`)
    (`BrainComponent.StartLogic` (`self.StateTree`))))

(event `ReturnToPool`
  ; Return to pool
  (`ActorComponent.K2_DestroyComponent` (`self.RoboticDeath`))
  (set `self.RoboticDeath` null)
  (`self.SetInUse` false)
  (`self.SetActorHiddenInGame` true))

(event `/Game/Game/Core/Interfaces/BPI_PooledActor.EV_ReturnToPool`
  ; Return to pool
  (`self.ReturnToPool`))

(fn `GiveAbilities`
  (for _array_element (`self.KnownAbilities`)
    (`AbilitySystemComponent.K2_GiveAbility` (`self.AbilitySystemComponent`) _array_element 0 -1)))

(fn `Initialize`
  (bind _uia_onfielddisplayhud (`self.UIA_OnFieldDisplayHUD`))
  (bind _asgs_game_state_game (cast `/Game/Game/Core/Blueprints/GameModes/GS_GameState_Game` (`GameplayStatics.GetGameState`))
    (:`then`
      (set `self.Gamestate` _asgs_game_state_game)
      (`AbilitySystemComponent.K2_InitStats` (`self.AbilitySystemComponent`) "/Script/GameOff25.BasicAttributeSet" null)
      (bind _returnvalue (`AbilitySystemBlueprintLibrary.MakeSpecHandleByClass` "/Game/Game/Core/Blueprints/Combatants/Abilities/Effects/GE_ChangeMaxHealth.GE_ChangeMaxHealth_C" null self))
      (bind _returnvalue_2 (`AbilitySystemBlueprintLibrary.AssignTagSetByCallerMagnitude` _returnvalue (struct :`TagName` "Data.MaxHealth") (`self.MaxHealth`)))
      (`AbilitySystemComponent.BP_ApplyGameplayEffectSpecToSelf` (`self.AbilitySystemComponent`) _returnvalue_2)
      (`self.CallAttributesInitialized`)
      (`self.GiveAbilities`)
      (`/Game/Game/Core/UI/Actors/UIA_OnFieldDisplayHUD.Initialize_UI` _uia_onfielddisplayhud "/Game/Game/Core/UI/Widgets/Widget_Assets/UIA_HealthBar_Enemy.UIA_HealthBar_Enemy_C")
      (`/Game/Game/Core/UI/Actors/UIA_OnFieldDisplayHUD.EditWidgetComponent` _uia_onfielddisplayhud "Screen" "Automatic" "Visible" false (75.0 100.0) (`KismetMathLibrary.MakeTransform` (25.0 0.0 0.0))))
    (:`CastFailed`
      (`KismetSystemLibrary.PrintString` "boss failed to cast to gamestate" true true (struct :`R` 1.0 :`B` 0.065357 :`A` 1.0) 600.0))))

(fn `ResetHealth`
  (bind _returnvalue (`AbilitySystemBlueprintLibrary.MakeSpecHandleByClass` "/Game/Game/Core/Blueprints/Combatants/Abilities/Effects/GE_ChangeMaxHealth.GE_ChangeMaxHealth_C" null self))
  (bind _returnvalue_2 (`AbilitySystemBlueprintLibrary.AssignTagSetByCallerMagnitude` _returnvalue (struct :`TagName` "Data.MaxHealth") (`self.MaxHealth`)))
  (`AbilitySystemComponent.BP_ApplyGameplayEffectSpecToSelf` (`self.AbilitySystemComponent`) _returnvalue_2))

(fn `UserConstructionScript`
  (`parent.UserConstructionScript`))