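; BP_DamagingCollision is an enemy component that deals contact damage through the owner's capsule and attaches a scout trail Niagara effect to it.
; On BeginPlay it destroys itself if the owner has another copy or lacks a capsule, otherwise it binds to capsule overlap.
; Overlaps skip the owner, same-class actors and bosses.
; Other ability system actors receive the hit instigator and a SetByCaller instant damage GameplayEffect, on authority only.
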(event `self.ReceiveBeginPlay`
  (bind _returnvalue (`Actor.GetComponentByClass` (`self.GetOwner`) "/Script/Engine.CapsuleComponent"))
  (if (> (`KismetArrayLibrary.Array_Length` (`Actor.K2_GetComponentsByClass` (`self.GetOwner`) "BP_DamagingCollision_C")) 1)
    (`self.K2_DestroyComponent` :!label _label)
    (else
      (`/Engine/EditorBlueprintResources/StandardMacros.IsValid` _returnvalue
        (:`Is Valid`
          (add `PrimitiveComponent.OnComponentBeginOverlap` _returnvalue (delegate `DoDamage`))
          (bind _returnvalue_2 (`|AddComponentByClass` :`self` (`self.GetOwner`) :`Class` "/Script/Niagara.NiagaraComponent"))
          (`NiagaraComponent.SetAsset` _returnvalue_2 "/Game/Game/Assets/Particles/NS_ScoutTrail.NS_ScoutTrail" true)
          (bind _output_get (set `self.Niagara` _returnvalue_2))
          (`SceneComponent.K2_AttachToComponent` _output_get _returnvalue "None" "SnapToTarget" "SnapToTarget" "SnapToTarget" true))
        (:`Is Not Valid`
          (goto _label))))))

(event `DoDamage`
  (params (OverlappedComponent :type "PrimitiveComponent Object Reference") (OtherActor :type "Actor Object Reference") (OtherComp :type "PrimitiveComponent Object Reference") (OtherBodyIndex :type Integer) (bFromSweep :type Boolean) (SweepResult :type "HitResult Structure (by ref)"))
  (if (!= OtherActor (`self.GetOwner`))
    ; Use collision channel instead?  Can enemies be set as pawn and antiplayer?
    (bind _ignoreactor_ (`self.ShouldActorBeIgnored?` OtherActor)) ; This should actually probably be done by collison channels
    (if (not _ignoreactor_)
      (`/Engine/EditorBlueprintResources/StandardMacros.IsValid` (`AbilitySystemBlueprintLibrary.GetAbilitySystemComponent` OtherActor)
        (:`Is Valid`
          (`self.ApplyDamage` OtherActor (`self.GetOwner`)))))))

(fn `ApplyDamage`
  (params (OtherActor :type "Actor Object Reference") (`Instigator Actor` :type "Actor Object Reference"))
  (bind _returnvalue (`AbilitySystemBlueprintLibrary.GetAbilitySystemComponent` OtherActor))
  ; GAS damage
  (`/Engine/EditorBlueprintResources/StandardMacros.IsValid` _returnvalue ; Does hit actor have ability system?
    (:`Is Valid`
      (`/Engine/EditorBlueprintResources/ActorComponentMacros.Switch Has Authority`
        (:`Authority`
          (message `/Game/Game/Core/Blueprints/Data/Interface/BPI_Player.Fn_Set_Current_HitInstigator` (`local.OtherActor`) (`local.Instigator Actor`))
          (bind _returnvalue_2 (`AbilitySystemBlueprintLibrary.MakeSpecHandleByClass` "/Game/Game/Core/Blueprints/Combatants/Abilities/Effects/GE_DamageInstant.GE_DamageInstant_C"))
          (bind _returnvalue_3 (`AbilitySystemBlueprintLibrary.AssignTagSetByCallerMagnitude` _returnvalue_2 (struct :`TagName` "Data.Damage") (`self.Damage`)))
          (`AbilitySystemComponent.BP_ApplyGameplayEffectSpecToSelf` _returnvalue _returnvalue_3))))))

(fn `ShouldActorBeIgnored?`
  (params (ActorToTest :type "Actor Object Reference"))
  (returns (`IgnoreActor?` :type Boolean))
  (bind _returnvalue (`GameplayStatics.GetObjectClass` ActorToTest))
  (return (or (== _returnvalue (`GameplayStatics.GetObjectClass` (`self.GetOwner`))) (`KismetMathLibrary.ClassIsChildOf` _returnvalue "/Game/Game/Core/Blueprints/Combatants/Enemy/BP_BossBase.BP_BossBase_C"))))