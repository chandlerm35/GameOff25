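; Base neutral destructible combatant that uses the Gameplay Ability System and awards score when destroyed.
; On BeginPlay it initializes attributes, applies max health via a SetByCaller effect, grants abilities and shows an enemy health bar.
; An attribute listener handles zero health, calling the empty OnDeathEffect hook, then passing a one-shot gate.
; The gate credits the instigator, adds score, spawns pooled score numbers, plays explosion audio, disables collision and adds a robotic death component.
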(event `self.ReceiveBeginPlay`
  (`parent.ReceiveBeginPlay`)
  (`self.Initialize`)
  (bind (_asynctaskproxy _attribute _newvalue) (`AbilityAsync_WaitAttributeChanged.WaitForAttributeChanged` null (struct :`AttributeName` "Health" :`Attribute` "/Script/GameOff25.BasicAttributeSet:Health" :`AttributeOwner` "/Script/CoreUObject.Class'/Script/GameOff25.BasicAttributeSet'")) ; This node can't be in a function
    (:`Changed`
      (`self.HandleHealthChanged` _newvalue))))

(event `HandleHealthChanged`
  (params (Health :type "Float (double-precision)"))
  ; Health Changed
  (if (<= Health 0.0)
    (`self.OnDeathEffect`)
    (`/Engine/EditorBlueprintResources/StandardMacros.Gate` false :!label _label
      (:`Exit`
        (`|ExecutionSequence`
          (:`then_0`
            (`|ExecutionSequence`
              (:`then_0`
                (`self.Fn_Defeated` (`self.Saved Hit Instigator`))
                ; Add points to score
                (message `/Game/Game/Core/Interfaces/BPI_GameState.Fn_AddScoreToCurrentScore` (`GameplayStatics.GetGameState`) (`self.PointValue`))
                (bind _pooledactor (`/Game/Game/Core/Blueprints/Components/AC_MultiObjectPool.SpawnFromPool` (`self.AC_UI Hit Numbers Pool`) (`self.GetTransform` self) "/Game/Game/Core/UI/Actors/UIA_HitNumbers.UIA_HitNumbers_C"))
                (message `/Game/Game/Core/Interfaces/BPI_UI_OnActor.Fn_Hit_ScoreSend` _pooledactor (`KismetMathLibrary.Conv_IntToDouble` (`self.PointValue`)) (`self.Saved Hit Instigator`)))
              (:`then_1`
                ;;[0.3193 0 1 0.5] SFX
                (`FMODBlueprintStatics.PlayEventAtLocation` "/Game/FMOD/Events/GameSFX/Explosions/MiniExplosion.MiniExplosion" (`KismetMathLibrary.MakeTransform` (`self.K2_GetActorLocation`)))
                ;; Remove components and explode
                (`self.SetActorEnableCollision` false)
                (`AddComponent|NODE_AddAC_RoboticDeath-0`))))
          (:`then_1`
            (goto _label :!via `Close`)))))))

(fn `GiveAbilities`
  (for _array_element (`self.KnownAbilities`)
    (`AbilitySystemComponent.K2_GiveAbility` (`self.AbilitySystemComponent`) _array_element 0 -1)))

(fn `Initialize`
  (bind _uia_onfielddisplayhud (`self.UIA_OnFieldDisplayHUD`))
  (bind _asgs_game_state_game (cast `/Game/Game/Core/Blueprints/GameModes/GS_GameState_Game` (`GameplayStatics.GetGameState`))
    (:`then`
      (set `self.Gamestate` _asgs_game_state_game)
      (`AbilitySystemComponent.K2_InitStats` (`self.AbilitySystemComponent`) "/Script/GameOff25.BasicAttributeSet" null)
      (bind _returnvalue (`AbilitySystemBlueprintLibrary.MakeSpecHandleByClass` "/Game/Game/Core/Blueprints/Combatants/Abilities/Effects/GE_ChangeMaxHealth.GE_ChangeMaxHealth_C" null self))
      (bind _returnvalue_2 (`AbilitySystemBlueprintLibrary.AssignTagSetByCallerMagnitude` _returnvalue (struct :`TagName` "Data.MaxHealth") (`self.MaxHealth`)))
      (`AbilitySystemComponent.BP_ApplyGameplayEffectSpecToSelf` (`self.AbilitySystemComponent`) _returnvalue_2)
      (`self.GiveAbilities`)
      (`/Game/Game/Core/UI/Actors/UIA_OnFieldDisplayHUD.Initialize_UI` _uia_onfielddisplayhud "/Game/Game/Core/UI/Widgets/Widget_Assets/UIA_HealthBar_Enemy.UIA_HealthBar_Enemy_C")
      (`/Game/Game/Core/UI/Actors/UIA_OnFieldDisplayHUD.EditWidgetComponent` _uia_onfielddisplayhud "Screen" "Automatic" "Visible" false (75.0 100.0) (`KismetMathLibrary.MakeTransform` (25.0 0.0 0.0))))
    (:`CastFailed`
      (`KismetSystemLibrary.PrintString` "neutralDestroy failed to cast to gamestate" true true (struct :`R` 1.0 :`B` 0.065357 :`A` 1.0) 600.0))))

(fn `OnDeathEffect`)

(fn `UserConstructionScript`
  (`parent.UserConstructionScript`))