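; Player state that tracks a player's defeated enemies and kill chain for scoring.
; Each defeat logs the enemy class, increments the chain, refills the chain timer and reports the count to the ACScoreSystem component for highest-chain checks.
; A looping timer event, rather than Tick, drains the chain timer and resets the chain when it runs out.
; Getters expose timer, chain and score system; debug prints trace activity.
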(event `self.ReceiveBeginPlay`
  (`KismetSystemLibrary.DelayUntilNextTick`)
  (bind _output_get (set `self.Possessed Actor` (`self.GetPawn`)))
  (`KismetSystemLibrary.PrintString` (`KismetTextLibrary.Conv_TextToString` (`|FormatText` "{a} has been created! Current Pawn: {b}" self _output_get)) true true (struct :`R` 1.0 :`G` 0.517657 :`A` 1.0) 15.0))

(event `/Game/Game/Core/Blueprints/Data/Interface/BPI_PlayerState_Game.Fn_DefeatedEnemy`
  (params (DefeatedEnemy :type "Actor Object Reference"))
  (`KismetArrayLibrary.Array_Add` (`self.DefeatedEnemy_List`) (`GameplayStatics.GetObjectClass` DefeatedEnemy))
  (`/Engine/EditorBlueprintResources/StandardMacros.IncrementInt` (`self.Chain Amount`)
    (:`  `
      (set `self.ChainTimer_Amount` 1.0)
      (bind _returnvalue (`KismetSystemLibrary.K2_SetTimerDelegate` (delegate `Loop_ChainKill`) 0.05 true true))
      (set `self.Loop_ChainTimer_Handle` _returnvalue)
      (`KismetSystemLibrary.PrintString` (`KismetTextLibrary.Conv_TextToString` (`|FormatText` "{a} has defeated {b}" (`self.GetPawn`) DefeatedEnemy)) true true (struct :`G` 0.859794 :`B` 1.0 :`A` 1.0) 2.0 "None")
      (`/Game/Game/Core/Blueprints/Components/AC_ScoreSystem.CheckHighestChain` (`self.AC_ScoreSystem`) (`self.Chain Amount`)))))

(event `Loop_ChainKill`
  (if (> (`self.ChainTimer_Amount`) 0.0)
    (bind _output_get (set `self.ChainTimer_Amount` (`KismetMathLibrary.FInterpTo` (`self.ChainTimer_Amount`) (- (`self.ChainTimer_Amount`) 0.02) 1.5 0.3)))
    (`KismetSystemLibrary.PrintString` (`KismetTextLibrary.Conv_TextToString` (`|FormatText` "Chain Time: {a}" _output_get)) true true (struct :`G` 1.0 :`B` 0.13257 :`A` 1.0) 2.0 "Chain")
    (else
      (set `self.ChainTimer_Amount` 0.0)
      (set `self.Chain Amount` 0)
      (`KismetSystemLibrary.K2_ClearAndInvalidateTimerHandle` (`self.Loop_ChainTimer_Handle`)))))

(fn `Fn_GetChainTimer`
  (returns (`Chain Timer Left` :type "Float (double-precision)"))
  (return (`self.ChainTimer_Amount`)))

(fn `Fn_GetCurrentChain`
  (returns (`Chain Amount` :type Integer))
  (return (`self.Chain Amount`)))

(fn `Fn_GetScoreSystem`
  (returns (`Score System` :type "/Game/Game/Core/Blueprints/Components/AC_ScoreSystem Object Reference"))
  (return (`self.AC_ScoreSystem`)))

(fn `UserConstructionScript`)