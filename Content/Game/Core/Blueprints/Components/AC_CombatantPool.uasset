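; Actor component that pre-spawns and pools wave combatants for reuse in place of spawning on demand.
; InitializePool tallies enemy classes from a wave spawn set, then spawns that many of each at the owner, skipping boss subclasses, into a class-keyed map.
; SpawnFromPool moves the first idle actor of the requested class, flags it in use and sends a spawn message.
; The pool never grows; failed lookups only print debug errors.
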(event `self.ReceiveBeginPlay`)

(fn `FindFirstAvalibleActorOfClass`
  (params (ClassToFind :type "/Game/Game/Core/Blueprints/Combatants/BP_CombatantBase Class Reference"))
  (returns (PooledActor :type "Actor Object Reference"))
  (bind (_value _returnvalue) (`BlueprintMapLibrary.Map_Find` (`self.ObjectPool`) (`local.ClassToFind`)))
  (bind _result (`|FormatText` "{owner} enemy pool tried to find an actor of class {class} which is not part of the pool." (`self.GetOwner`) (`KismetSystemLibrary.GetClassDisplayName` ClassToFind)))
  (if (`BlueprintMapLibrary.Map_Contains` (`self.PooledEnemiesNeededToSpawn`) ClassToFind)
    (if _returnvalue
      (for _array_element (`.ListofCombatantsSaved_3_DCB73E0343AE76C3BEFE89817A62A978` (break `/Game/Game/Core/Blueprints/Data/Structs/S_Wave_PooledActorsList` _value))
        (bind _in_use_ (message `/Game/Game/Core/Interfaces/BPI_PooledActor.Fn_GetInUse` _array_element))
        (if (not _in_use_)
          (return _array_element))))
    (else
      (`KismetSystemLibrary.PrintString` (`KismetTextLibrary.Conv_TextToString` _result) true true (struct :`R` 1.0 :`G` 0.00584 :`A` 1.0) 60.0 (`KismetStringLibrary.Conv_StringToName` (`KismetTextLibrary.Conv_TextToString` _result))))))

(fn `Initialize Pool`
  (params (`Wave Sets to Spawn` :type "/Game/Game/Core/Blueprints/Data/Structs/S_WaveSpawn_Set Structure"))
  ; Step 1: Set amount needed to spawn
  (`self.Initialize Pool Needed To Spawn` `Wave Sets to Spawn`)
  ; Checks current Pooled Enemy info list
  (bind _keys (`BlueprintMapLibrary.Map_Keys` (`self.PooledEnemiesNeededToSpawn`)))
  (for _array_element _keys
    (if (`KismetSystemLibrary.IsValidClass` _array_element)
      ; Basically makes the listing to call each actor class if missing from Object Pool
      (if (not (`BlueprintMapLibrary.Map_Contains` (`self.ObjectPool`) _array_element))
        (`BlueprintMapLibrary.Map_Add` (`self.ObjectPool`) _array_element)
        (`KismetSystemLibrary.PrintString` (`KismetTextLibrary.Conv_TextToString` (`|FormatText` "Adding class {a} to Object Pool." (`KismetSystemLibrary.GetClassDisplayName` _array_element))) true true (struct :`R` 1.0 :`G` 0.235508 :`B` 0.014647 :`A` 1.0) 60.0))
      (else
        (bind _result (`|FormatText` "{owner} Multipool tried to spawn invalid class {Class}" (`self.GetOwner`) (`KismetSystemLibrary.GetClassDisplayName` _array_element)))
        ; If Actor Class trying to spawn is invalid..
        (`KismetSystemLibrary.PrintString` (`KismetTextLibrary.Conv_TextToString` _result) true true (struct :`R` 1.0 :`G` 0.316174 :`A` 1.0) 60.0 (`KismetStringLibrary.Conv_StringToName` (`KismetTextLibrary.Conv_TextToString` _result))))))
  ; Step 2: Go through each Class and spawn the amount needed and add it to their array
  (bind _keys_2 (`BlueprintMapLibrary.Map_Keys` (`self.PooledEnemiesNeededToSpawn`)))
  (for _array_element_2 _keys_2
    (`self.Initialize Spawn Pool Objects` _array_element_2)))

(fn `Initialize Pool Needed To Spawn`
  (params (S_WaveSpawn_Set :type "/Game/Game/Core/Blueprints/Data/Structs/S_WaveSpawn_Set Structure (by ref)"))
  (locals (ClassActors_NeedToSpawn :type "Map of /Game/Game/Core/Blueprints/Combatants/BP_CombatantBase Class Reference to Integer"))
  (bind _classactors_needtospawn (`local.ClassActors_NeedToSpawn`))
  (for _array_element (`.Enemiestospawnlist_3_A0D966784CC86F605833DD8363EDC8C6` (break `/Game/Game/Core/Blueprints/Data/Structs/S_WaveSpawn_Set` S_WaveSpawn_Set))
    (bind _actorstospawn (break `/Game/Game/Core/Blueprints/Data/Structs/S_WaveSpawn` _array_element))
    (bind (_value _returnvalue) (`BlueprintMapLibrary.Map_Find` _classactors_needtospawn _actorstospawn))
    (if _returnvalue
      (bind _result (`/Engine/EditorBlueprintResources/StandardMacros.IncrementInt` _value)
        (:`  `
          ; If already present, add to number
          (`BlueprintMapLibrary.Map_Add` _classactors_needtospawn _actorstospawn _result)
          (bind _returnvalue_2 (`KismetSystemLibrary.GetClassDisplayName` _actorstospawn))
          (`KismetSystemLibrary.PrintString` (`KismetTextLibrary.Conv_TextToString` (`|FormatText` "Adding class {a} to spawn pool. Current Stacks: {b}" _returnvalue_2 _result)) true true (struct :`R` 0.375956 :`G` 0.411576 :`B` 1.0 :`A` 1.0) 60.0 (`KismetStringLibrary.Conv_StringToName` _returnvalue_2))))
      (else
        ; If not already counted, make new key
        (`BlueprintMapLibrary.Map_Add` _classactors_needtospawn _actorstospawn 1))))
  (set `self.PooledEnemiesNeededToSpawn` (`local.ClassActors_NeedToSpawn`)))

(fn `Initialize Spawn Pool Objects`
  (params (`Combatant Class to Spawn` :type "/Game/Game/Core/Blueprints/Combatants/BP_CombatantBase Class Reference"))
  (locals (CombatantsSpawned_Array :type "Array of /Game/Game/Core/Blueprints/Combatants/BP_CombatantBase Object Reference"))
  (bind (_value _returnvalue) (`BlueprintMapLibrary.Map_Find` (`self.PooledEnemiesNeededToSpawn`) `Combatant Class to Spawn`))
  (if _returnvalue
    (for _ (range _value)
      (if (not (`KismetMathLibrary.ClassIsChildOf` `Combatant Class to Spawn` "/Game/Game/Core/Blueprints/Combatants/Enemy/BP_BossBase.BP_BossBase_C"))
        (bind _returnvalue_2 (`|SpawnActorFromClass` `Combatant Class to Spawn` (`Actor.GetTransform` (`self.GetOwner`)) "Undefined" "MultiplyWithRoot" (`self.GetOwner`) null))
        (bind _returnvalue_3 (`KismetArrayLibrary.Array_Add` (`local.CombatantsSpawned_Array`) _returnvalue_2))
        (message `/Game/Game/Core/Interfaces/BPI_PooledActor.Fn_SetInUse` _returnvalue_2 false)))
    (`KismetSystemLibrary.PrintString` (`KismetTextLibrary.Conv_TextToString` (`|FormatText` "Finishing spawning all of class {a} / Total: {b}" (`KismetSystemLibrary.GetClassDisplayName` (`local.Combatant Class to Spawn`)) (`KismetArrayLibrary.Array_Length` (`local.CombatantsSpawned_Array`)))) true true (struct :`R` 1.0 :`G` 0.228533 :`B` 0.941518 :`A` 1.0) 60.0)
    (`BlueprintMapLibrary.Map_Add` (`self.ObjectPool`) (`local.Combatant Class to Spawn`) (make `/Game/Game/Core/Blueprints/Data/Structs/S_Wave_PooledActorsList` (`local.CombatantsSpawned_Array`)))))

(fn `SpawnFromPool`
  (params (SpawnTransform :type "Transform Structure") (ClassToSpawn :type "/Game/Game/Core/Blueprints/Combatants/BP_CombatantBase Class Reference"))
  (returns (PooledActor :type "Actor Object Reference"))
  (bind _pooledactor (`self.FindFirstAvalibleActorOfClass` ClassToSpawn))
  (`/Engine/EditorBlueprintResources/StandardMacros.IsValid` _pooledactor
    (:`Is Valid`
      (`Actor.K2_SetActorTransform` _pooledactor SpawnTransform false false)
      (message `/Game/Game/Core/Interfaces/BPI_PooledActor.Fn_SetInUse` _pooledactor true)
      (message `/Game/Game/Core/Blueprints/Data/Interface/BPI_Player.Ev_OnSpawn` _pooledactor)
      (return _pooledactor))
    (:`Is Not Valid`
      ;[1 1 1] If this goes off either the pool is empty or something went wrong.  Maybe make a system where the pool can dynamically grow and then shrink if the average pool use lowers again?
      (`KismetSystemLibrary.PrintString` (`KismetTextLibrary.Conv_TextToString` (`|FormatText` "{Owner} failed to find pooled actor not in use of type {pooled object}.  Please check the pool size." (`self.GetOwner`) (`KismetSystemLibrary.GetClassDisplayName` (`local.ClassToSpawn`)))) true true (struct :`R` 1.0 :`G` 0.00584 :`A` 1.0) 60.0 (`KismetStringLibrary.Conv_StringToName` (`KismetTextLibrary.Conv_TextToString` (`|FormatText` "{class} Pooled Object Spawn Error " (`self.GetOwner`))))))))