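; Actor component that pools enemies of several classes for reuse by its owner.
; On BeginPlay it spawns the configured count of each class in the PooledEnemies map at the owner's transform and marks them not in use.
; SpawnFromPool finds a free actor of the requested class, moves it, marks it in use and calls its OnSpawn.
; The pool never grows; exhausted pools and invalid or unknown classes print on-screen errors.
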(event `self.ReceiveBeginPlay`
  (`self.InitializePool`))

(event `InitializePool`
  ; Multipool spawning
  (bind _keys (`BlueprintMapLibrary.Map_Keys` (`self.PooledEnemies`)))
  (for _array_element _keys
    (if (`KismetSystemLibrary.IsValidClass` _array_element)
      (for _ (range (+ (`BlueprintMapLibrary.Map_Find` (`self.PooledEnemies`) _array_element) 1))
        (bind _returnvalue (`|SpawnActorFromClass` _array_element (`Actor.GetTransform` (`self.GetOwner`)) "Undefined" "MultiplyWithRoot" (`self.GetOwner`) null))
        (`KismetArrayLibrary.Array_AddUnique` (`self.ObjectPool`) _returnvalue)
        (`/Game/Game/Core/Blueprints/Combatants/Enemy/BP_EnemyBase.SetInUse` _returnvalue false))
      (else
        (bind _result (`|FormatText` "{owner} Multipool tried to spawn invalid class {Class}" (`self.GetOwner`) (`KismetSystemLibrary.GetClassDisplayName` _array_element)))
        (`KismetSystemLibrary.PrintString` (`KismetTextLibrary.Conv_TextToString` _result) true true (struct :`R` 1.0 :`B` 0.00682 :`A` 1.0) 60.0 (`KismetStringLibrary.Conv_StringToName` (`KismetTextLibrary.Conv_TextToString` _result)))))))

(fn `FindFirstAvalibleActor`
  (returns (PooledActor :type "/Game/Game/Core/Blueprints/Combatants/Enemy/BP_EnemyBase Object Reference"))
  (for _array_element (`self.ObjectPool`)
    (if (not (`/Game/Game/Core/Blueprints/Combatants/Enemy/BP_EnemyBase.InUse` _array_element))
      (return _array_element))))

(fn `FindFirstAvalibleActorOfClass`
  (params (ClassToFind :type "/Game/Game/Core/Blueprints/Combatants/Enemy/BP_EnemyBase Class Reference"))
  (returns (PooledActor :type "/Game/Game/Core/Blueprints/Combatants/Enemy/BP_EnemyBase Object Reference"))
  (bind _result (`|FormatText` "{owner} enemy pool tried to find an actor of class {class} which is not part of the pool." (`self.GetOwner`) (`KismetSystemLibrary.GetClassDisplayName` ClassToFind)))
  (bind _keys (`BlueprintMapLibrary.Map_Keys` (`self.PooledEnemies`)))
  (if (`KismetArrayLibrary.Array_Contains` _keys ClassToFind)
    (for _array_element (`self.ObjectPool`)
      (bind _classtofind (`local.ClassToFind`)
        (:`then`
          (if (== (`GameplayStatics.GetObjectClass` _array_element) _classtofind)
            (if (`KismetSystemLibrary.IsValid` _array_element)
              (if (not (`/Game/Game/Core/Blueprints/Combatants/Enemy/BP_EnemyBase.InUse` _array_element))
                (return _array_element)))))
        (:`else`)))
    (else
      (`KismetSystemLibrary.PrintString` (`KismetTextLibrary.Conv_TextToString` _result) true true (struct :`R` 1.0 :`G` 0.00584 :`A` 1.0) 60.0 (`KismetStringLibrary.Conv_StringToName` (`KismetTextLibrary.Conv_TextToString` _result))))))

(fn `SpawnFromPool`
  (params (SpawnTransform :type "Transform Structure") (ClassToSpawn :type "/Game/Game/Core/Blueprints/Combatants/Enemy/BP_EnemyBase Class Reference"))
  (returns (PooledActor :type "/Game/Game/Core/Blueprints/Combatants/Enemy/BP_EnemyBase Object Reference"))
  (bind _pooledactor (`self.FindFirstAvalibleActorOfClass` ClassToSpawn))
  (`/Engine/EditorBlueprintResources/StandardMacros.IsValid` _pooledactor
    (:`Is Valid`
      (`Actor.K2_SetActorTransform` _pooledactor SpawnTransform false false)
      (`/Game/Game/Core/Blueprints/Combatants/Enemy/BP_EnemyBase.SetInUse` _pooledactor true)
      (`/Game/Game/Core/Blueprints/Combatants/Enemy/BP_EnemyBase.OnSpawn` _pooledactor)
      (return _pooledactor))
    (:`Is Not Valid`
      ;[1 1 1] If this goes off either the pool is empty or something went wrong.  Maybe make a system where the pool can dynamically grow and then shrink if the average pool use lowers again?
      (`KismetSystemLibrary.PrintString` (`KismetTextLibrary.Conv_TextToString` (`|FormatText` "{Owner} failed to find pooled actor not in use of type {pooled object}.  Please check the pool size." (`self.GetOwner`) (`KismetSystemLibrary.GetClassDisplayName` (`local.ClassToSpawn`)))) true true (struct :`R` 1.0 :`G` 0.00584 :`A` 1.0) 60.0 (`KismetStringLibrary.Conv_StringToName` (`KismetTextLibrary.Conv_TextToString` (`|FormatText` "{class} Pooled Object Spawn Error " (`self.GetOwner`))))))))