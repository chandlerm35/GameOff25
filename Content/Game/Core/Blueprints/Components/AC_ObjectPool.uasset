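; Actor component that pre-spawns and reuses actors of a configurable class for its owner.
; On BeginPlay it fills the pool at the owner's transform, marking each actor not in use.
; SpawnFromPool linearly searches for the first free actor, moves it to the requested transform, marks it in use and calls SpawnedIn.
; The pool never grows, so exhaustion or a missing class only prints an error.
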(event `self.ReceiveBeginPlay`
  (`self.InitializePool`))

(event `InitializePool`
  (bind _returnvalue (`self.GetOwner`))
  (for _ (range (+ (`self.PoolSize`) 1))
    (`self.PooledActorClass`
      (:`then`
        (bind _returnvalue_2 (`|SpawnActorFromClass` (`self.PooledActorClass`) (`Actor.GetTransform` (`self.GetOwner`)) "Undefined" "MultiplyWithRoot" _returnvalue 5.0 (cast `Pawn` _returnvalue :!pure true)))
        (`KismetArrayLibrary.Array_AddUnique` (`self.ObjectPool`) _returnvalue_2)
        (`/Game/Game/Core/Blueprints/Actors/BP_PooledActor.SetInUse` _returnvalue_2 false))
      (:`else`
        (`KismetSystemLibrary.PrintString` (`KismetTextLibrary.Conv_TextToString` (`|FormatText` "{Blueprint Name} tried to initilize an object pool, but the pooled actor is null." (`self.GetOwner`))) true true (struct :`R` 1.0 :`B` 0.1793 :`A` 1.0) 30.0 "Pooled Actor Null")))))

(fn `FindFirstAvalibleActor`
  (returns (PooledActor :type "/Game/Game/Core/Blueprints/Actors/BP_PooledActor Object Reference"))
  (for _array_element (`self.ObjectPool`)
    (if (not (`/Game/Game/Core/Blueprints/Actors/BP_PooledActor.InUse` _array_element))
      (return _array_element))))

(fn `SpawnFromPool`
  (params (SpawnTransform :type "Transform Structure"))
  (returns (PooledActor :type "/Game/Game/Core/Blueprints/Actors/BP_PooledActor Object Reference"))
  (bind _pooledactor (`self.FindFirstAvalibleActor`))
  (`/Engine/EditorBlueprintResources/StandardMacros.IsValid` _pooledactor
    (:`Is Valid`
      (`Actor.K2_SetActorTransform` _pooledactor SpawnTransform false false)
      (`/Game/Game/Core/Blueprints/Actors/BP_PooledActor.SetInUse` _pooledactor true)
      (`self.SpawnedIn` _pooledactor)
      (return _pooledactor))
    (:`Is Not Valid`
      ;[1 1 1] If this goes off either the pool is empty or something went wrong.  Maybe make a system where the pool can dynamically grow and then shrink if the average pool use lowers again?
      (`KismetSystemLibrary.PrintString` (`KismetTextLibrary.Conv_TextToString` (`|FormatText` "{Owner} failed to find pooled actor not in use of type {pooled object}.  Please check the pool size." (`self.GetOwner`) (`KismetSystemLibrary.GetClassDisplayName` (`self.PooledActorClass`)))) true true (struct :`R` 1.0 :`G` 0.00584 :`A` 1.0) 30.0 "Pooled Object Spawn Error"))))