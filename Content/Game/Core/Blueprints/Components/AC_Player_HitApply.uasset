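; Actor component on the player that applies and ends hit stop when the owner is hit.
; CallHitPause converts the incoming HitStop value into a duration by scaling it and adding a small base, then calls PlayerHitStopApply on the owner with the damage causer and type.
; CallEndHitPause ends the pause through PlayerEndHitstop on the owner.
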(fn CallHitPause
  (params (Damage%20Causer :type Actor%20Object%20Reference) (Damage%20Type :type Damage%20Type%20Class%20Reference) (Hit%20Stop :type Float%20%28double-precision%29))
  (CallFunction|PlayerHitStopApply (|((X*0.010000)+Y) Hit%20Stop 0.1) (Components|GetOwner) Damage%20Causer Damage%20Type))

(fn CallEndHitPause
  (CallFunction|PlayerEndHitstop (Components|GetOwner)))