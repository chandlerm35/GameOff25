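; Actor component that plays a robotic death sequence on its owner, starting at BeginPlay.
; It applies a generic flash material to the first skeletal or static mesh found, then starts a looping shake timer.
; Shakes jitter the mesh, nudge the actor backward and periodically spawn small explosions within its bounds.
; After a delay, a large explosion spawns and the owner returns to its pool if supported, otherwise is destroyed.
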(event `self.ReceiveBeginPlay`
  (bind _returnvalue (`self.GetOwner`))
  (bind _flashedcomponent (`self.FlashedComponent`))
  (bind _returnvalue_2 (`Actor.GetComponentByClass` (`self.GetOwner`) "/Script/Engine.SkeletalMeshComponent"))
  (bind _returnvalue_3 (`Actor.GetComponentByClass` (`self.GetOwner`) "/Script/Engine.StaticMeshComponent"))
  ; Initialize
  (`/Engine/EditorBlueprintResources/StandardMacros.IsValid` (`self.Owner`)
    (:`Is Not Valid`
      (set `self.Owner` (`self.GetOwner`))
      (bind _output_get (set `self.MeshComponent` (`Actor.GetComponentByClass` (`self.Owner`) "/Script/Engine.MeshComponent")))
      (set `self.InitialComponentLocation` (`SceneComponent.RelativeLocation` _output_get))
      ; Get and validate mesh
      (`/Engine/EditorBlueprintResources/StandardMacros.IsValid` _returnvalue_2
        (:`Is Valid`
          (set `self.FlashedComponent` _returnvalue_2)
          ; Initialize generic flash material
          (set `self.OriginalMaterial` (`PrimitiveComponent.GetMaterial` _flashedcomponent 0) :!label _label)
          (bind _returnvalue_4 (`PrimitiveComponent.CreateDynamicMaterialInstance` _flashedcomponent 0 "/Game/Game/Assets/Characters/M_GenericFlash.M_GenericFlash" "None"))
          (bind _output_get_2 (set `self.FlashMaterial` _returnvalue_4))
          (`MaterialInstanceDynamic.SetVectorParameterValue` _output_get_2 "FlashColor" (`self.FlashColor`))
          (`MaterialInstanceDynamic.SetScalarParameterValue` _output_get_2 "FlashIntensity" (`self.FlashIntensity`))
          ; Shakes and explosion
          (`KismetSystemLibrary.K2_SetTimerDelegate` (`|CreateDelegate` :!event `Shake`) (/ 0.5 (`self.ShakeFrequency`)) true true)
          (`KismetSystemLibrary.Delay` (`self.TimeUntilDeath`))
          (`NiagaraFunctionLibrary.SpawnSystemAtLocation` "/Game/Game/Assets/Particles/NS_LargeExplosion.NS_LargeExplosion" (`Actor.K2_GetActorLocation` _returnvalue) (struct) (3.0 3.0 3.0))
          (if (`KismetSystemLibrary.DoesImplementInterface` _returnvalue "/Game/Game/Core/Interfaces/BPI_PooledActor.BPI_PooledActor_C")
            (message `/Game/Game/Core/Interfaces/BPI_PooledActor.EV_ReturnToPool` _returnvalue)
            (else
              (`Actor.K2_DestroyActor` _returnvalue))))
        (:`Is Not Valid`
          (`/Engine/EditorBlueprintResources/StandardMacros.IsValid` _returnvalue_3
            (:`Is Valid`
              (set `self.FlashedComponent` _returnvalue_3)
              (goto _label))
            (:`Is Not Valid`
              ; Print warning if no mesh was found.
              (`KismetSystemLibrary.PrintString` (`KismetTextLibrary.Conv_TextToString` (`|FormatText` "{Component} on {Owner Display Name} failed to get static mesh or skeletal mesh" (`KismetSystemLibrary.GetClassDisplayName` (`GameplayStatics.GetObjectClass` self)) (`KismetSystemLibrary.GetDisplayName` (`self.Owner`))))))))))))

(event `Shake`
  (bind (_origin _boxextent) (`Actor.GetActorBounds` (`self.GetOwner`) false false))
  (`Actor.K2_AddActorLocalOffset` (`self.GetOwner`) (-2.0 0.0 0.0) false false)
  (`SceneComponent.K2_SetRelativeLocation` (`self.MeshComponent`) (+ (`self.InitialComponentLocation`) (* (`KismetMathLibrary.RotateAngleAxis` (1.0 0.0 0.0) (* (`KismetMathLibrary.RandomFloat`) 360.0) (0.0 0.0 1.0)) (`self.ShakeIntensity`))) false true)
  (bind _result (`/Engine/EditorBlueprintResources/StandardMacros.IncrementInt` (`self.ShakeCount`))
    (:`  `
      (if (== (mod _result 4) 0)
        (`NiagaraFunctionLibrary.SpawnSystemAtLocation` "/Game/Game/Assets/Particles/NS_Explosion.NS_Explosion" (+ _origin (* (`KismetMathLibrary.RandomUnitVector`) (`KismetMathLibrary.VSize` _boxextent) 0.5) (-50.0 0.0 0.0)) (struct) (0.01 0.01 0.01))))))