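; Score component that tracks a player's feats during play and turns them into end bonuses defined in a score bonus data table.
; It watches owner attribute changes through GAS for lowest health, records highest chain via CheckHighestChain, and counts upgrade purchases.
; CalculateBonusesForPlayer collects rows earned by chain and low-health thresholds, then sends the summed bonus to GameState.
; A looping timer queries the current chain but leaves the result unused.
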(event `self.ReceiveBeginPlay`
  (bind _returnvalue (`AbilitySystemBlueprintLibrary.GetAbilitySystemComponent` (`self.GetOwner`)))
  (bind (_bsuccessfullyfoundattribute _returnvalue_2) (`AbilitySystemBlueprintLibrary.GetFloatAttributeFromAbilitySystemComponent` _returnvalue (struct :`AttributeName` "MaxHealth" :`Attribute` "/Script/GameOff25.BasicAttributeSet:MaxHealth" :`AttributeOwner` "/Script/CoreUObject.Class'/Script/GameOff25.BasicAttributeSet'")))
  (`self.Initialize Bonuses Data Table List` "/Game/Game/Core/Blueprints/Data/ScoreBonuses/DT_ScoreBonus_List.DT_ScoreBonus_List")
  (`/Engine/EditorBlueprintResources/StandardMacros.IsValid` _returnvalue
    (:`Is Valid`
      (`|ExecutionSequence`
        (:`then_0`
          (bind (_asynctaskproxy _attribute _newvalue) (`AbilityAsync_WaitAttributeChanged.WaitForAttributeChanged` (`self.GetOwner`) (struct :`AttributeName` "Health" :`Attribute` "/Script/GameOff25.BasicAttributeSet:Health" :`AttributeOwner` "/Script/CoreUObject.Class'/Script/GameOff25.BasicAttributeSet'"))
            (:`Changed`
              (if _bsuccessfullyfoundattribute
                (`self.CheckLowestHealth` _newvalue _returnvalue_2)))))))))

(event `Restart_Loop`
  (bind _returnvalue (`KismetSystemLibrary.K2_SetTimerDelegate` (delegate `Loop_Calculate`) 0.03 true true))
  (set `self.Loop_Main` _returnvalue))

(event `Loop_Calculate`
  (bind _player_state (message `/Game/Game/Core/Blueprints/Data/Interface/BPI_Player.Fn_Get_Pawn_PlayerState` (`self.GetOwner`)))
  (message `/Game/Game/Core/Blueprints/Data/Interface/BPI_PlayerState_Game.Fn_GetCurrentChain` _player_state))

(fn `Add Upgrades Bought`
  (`|ExecutionSequence`
    (:`then_0`
      (bind _returnvalue (`|GetDataTableRow` (`self.Score Bonus DT`) "5")
        (:`then`
          (`KismetArrayLibrary.Array_AddUnique` (`self.ScoreBonus_Attained`) _returnvalue)
          (`KismetSystemLibrary.PrintString` "Bought an upgrade... adding to score")
          (bind _result (`/Engine/EditorBlueprintResources/StandardMacros.IncrementInt` (`self.UpgradeAmt`))
            (:`  `
              (set `self.UpgradeAmt` _result))))))
    (:`then_1`
      (if (>= (`self.UpgradeAmt`) 5)
        (bind _returnvalue_2 (`|GetDataTableRow` (`self.Score Bonus DT`) "6")
          (:`then`
            (`KismetArrayLibrary.Array_AddUnique` (`self.ScoreBonus_Attained`) _returnvalue_2)))))))

(fn `Calculate Bonuses for Player`
  (returns (`Bonuses Attained` :type "Array of /Game/Game/Core/Blueprints/Data/Structs/S_ScoreBonus Structure"))
  (locals (BonusesAttained_List :type "Array of /Game/Game/Core/Blueprints/Data/Structs/S_ScoreBonus Structure") (BonusScore_Total :type Integer))
  (`|ExecutionSequence`
    (:`then_0`
      (`self.Initialize Bonuses Data Table List` "/Game/Game/Core/Blueprints/Data/ScoreBonuses/DT_ScoreBonus_List.DT_ScoreBonus_List"))
    (:`then_1`
      (if (> (`KismetArrayLibrary.Array_Length` (`self.ScoreBonus_TOTAL_List`)) 0)
        (`|ExecutionSequence`
          (:`then_0`
            ; Check for chains
            (if (>= (`self.Chain_HighestAmount`) 20)
              (bind _returnvalue (`|GetDataTableRow` (`self.Score Bonus DT`) "2")
                (:`then`
                  (`KismetArrayLibrary.Array_AddUnique` (`self.ScoreBonus_Attained`) _returnvalue))
                (:`RowNotFound`
                  _)))
            (if (>= (`self.Chain_HighestAmount`) 10)
              (bind _returnvalue_2 (`|GetDataTableRow` (`self.Score Bonus DT`) "1")
                (:`then`
                  (`KismetArrayLibrary.Array_AddUnique` (`self.ScoreBonus_Attained`) _returnvalue_2))
                (:`RowNotFound`
                  _)))
            (if (>= (`self.Chain_HighestAmount`) 5)
              (bind _returnvalue_3 (`|GetDataTableRow` (`self.Score Bonus DT`) "0")
                (:`then`
                  (`KismetArrayLibrary.Array_AddUnique` (`self.ScoreBonus_Attained`) _returnvalue_3)))))
          (:`then_1`
            ; Low Health Completion
            (if (<= (`self.Health_LowestPercentage`) 0.25)
              (bind _returnvalue_4 (`|GetDataTableRow` (`self.Score Bonus DT`) "3")
                (:`then`
                  (`KismetArrayLibrary.Array_AddUnique` (`self.ScoreBonus_Attained`) _returnvalue_4)))))
          (:`then_2`
            (for _array_element (`local.BonusesAttained_List`)
              (set `local.BonusScore_Total` (+ (`local.BonusScore_Total`) (`.ScoreAmount_6_0BB4E261419F767E40BBA889C35D3807` (break `/Game/Game/Core/Blueprints/Data/Structs/S_ScoreBonus` _array_element)))))
            (message `/Game/Game/Core/Interfaces/BPI_GameState.Fn_AddScoreToCurrentScore` (`GameplayStatics.GetGameState`) (`local.BonusScore_Total`))
            (return (`self.ScoreBonus_Attained`))))))))

(fn `CheckHighestChain`
  (params (`Chain Amount to Compare` :type Integer))
  (if (>= `Chain Amount to Compare` (`self.Chain_HighestAmount`))
    (set `self.Chain_HighestAmount` (`local.Chain Amount to Compare`))))

(fn `CheckLowestHealth`
  (params (`New Health` :type "Float (double-precision)") (`Max Health` :type "Float (double-precision)"))
  (if (<= (/ `New Health` `Max Health`) (`self.Health_LowestPercentage`))
    (set `self.Health_LowestPercentage` (`local.New Health`))))

(fn `Initialize Bonuses Data Table List`
  (params (`Data Table` :type "DataTable Object Reference"))
  (locals (DT_RowNames :type "Array of Name"))
  (`/Engine/EditorBlueprintResources/StandardMacros.IsValid` `Data Table`
    (:`Is Valid`
      (set `self.Score Bonus DT` `Data Table`)
      ; Clear current list and read the new DT data
      (`/Engine/EditorBlueprintResources/StandardMacros.IsValid` (`self.Score Bonus DT`)
        (:`Is Valid`
          (`KismetArrayLibrary.Array_Clear` (`self.ScoreBonus_TOTAL_List`))
          (bind _outrownames (`DataTableFunctionLibrary.GetDataTableRowNames` (`self.Score Bonus DT`)))
          (bind _output_get (set `local.DT_RowNames` _outrownames))
          (for _array_element _output_get
            ; Add Spawn list to array
            (bind _returnvalue (`|GetDataTableRow` (`self.Score Bonus DT`) _array_element)
              (:`then`
                (`KismetArrayLibrary.Array_AddUnique` (`self.ScoreBonus_TOTAL_List`) _returnvalue)))))))))