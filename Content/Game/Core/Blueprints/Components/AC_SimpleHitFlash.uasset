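; Actor component that briefly flashes its owner's mesh when the owner takes damage, with optional Niagara impact particles.
; InitializeHitFlash binds to damage and prepares a generic flash material for the first skeletal, otherwise static, mesh found.
; DamageFlash swaps material slot 0 for a set duration, skipping hits mid-flash.
; Particles randomly pick circular or causer-angled bursts as a placeholder; the older emissive-parameter graph is unused.
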(event `Initialize Hit Flash`
  (bind _returnvalue (`self.GetOwner`))
  (bind _flashedcomponent (`self.FlashedComponent`))
  (bind _returnvalue_2 (`Actor.GetComponentByClass` (`self.GetOwner`) "/Script/Engine.SkeletalMeshComponent"))
  (bind _returnvalue_3 (`Actor.GetComponentByClass` (`self.GetOwner`) "/Script/Engine.StaticMeshComponent"))
  ; Initialize
  (`/Engine/EditorBlueprintResources/StandardMacros.IsValid` (`self.Owner`)
    (:`Is Not Valid`
      (set `self.Owner` _returnvalue)
      (add `Actor.OnTakeAnyDamage` _returnvalue (`|CreateDelegate` :!event `DamageFlash`))
      ; Get and validate mesh
      (`/Engine/EditorBlueprintResources/StandardMacros.IsValid` _returnvalue_2
        (:`Is Valid`
          (set `self.FlashedComponent` _returnvalue_2)
          ; Initialize generic flash material
          (set `self.OriginalMaterial` (`PrimitiveComponent.GetMaterial` _flashedcomponent 0) :!label _label)
          (bind _returnvalue_4 (`PrimitiveComponent.CreateDynamicMaterialInstance` _flashedcomponent 0 "/Game/Game/Assets/Characters/M_GenericFlash.M_GenericFlash" "None"))
          (bind _output_get (set `self.FlashMaterial` _returnvalue_4))
          (`MaterialInstanceDynamic.SetVectorParameterValue` _output_get "FlashColor" (`self.FlashColor`))
          (`MaterialInstanceDynamic.SetScalarParameterValue` _output_get "FlashIntensity" (`self.FlashIntensity`))
          (`PrimitiveComponent.SetMaterial` (`self.FlashedComponent`) 0 (`self.OriginalMaterial`)))
        (:`Is Not Valid`
          (`/Engine/EditorBlueprintResources/StandardMacros.IsValid` _returnvalue_3
            (:`Is Valid`
              (set `self.FlashedComponent` _returnvalue_3)
              (goto _label))
            (:`Is Not Valid`
              ; Print warning if no mesh was found.
              (`KismetSystemLibrary.PrintString` (`KismetTextLibrary.Conv_TextToString` (`|FormatText` "{Component} on {Owner Display Name} failed to get static mesh or skeletal mesh" (`KismetSystemLibrary.GetClassDisplayName` (`GameplayStatics.GetObjectClass` self)) (`KismetSystemLibrary.GetDisplayName` (`self.Owner`))))))))))))

(event `DamageFlash`
  (params (DamagedActor :type "Actor Object Reference") (Damage :type "Float (single-precision)") (DamageType :type "DamageType Object Reference") (InstigatedBy :type "Controller Object Reference") (DamageCauser :type "Actor Object Reference"))
  (bind _flashedcomponent (`self.FlashedComponent`))
  ; Set flash material
  (if (not (== (`PrimitiveComponent.GetMaterial` _flashedcomponent 0) (`self.FlashMaterial`)))
    (`PrimitiveComponent.SetMaterial` _flashedcomponent 0 (`self.FlashMaterial`))
    (if (`self.SpawnParticles`)
      ; Randomize (placeholder for final implementation of directional hits)
      (if (`KismetMathLibrary.RandomBool`)
        ; Hit particles (circular)
        (`NiagaraFunctionLibrary.SpawnSystemAtLocation` "/Game/Game/Assets/Particles/NS_SmallImpact.NS_SmallImpact" (`Actor.GetActorBounds` DamagedActor true false) :!label _label_2)
        (else
          (`/Engine/EditorBlueprintResources/StandardMacros.IsValid` DamageCauser
            (:`Is Valid`
              ; Hit particles (directional)
              (bind _returnvalue (`NiagaraFunctionLibrary.SpawnSystemAtLocation` "/Game/Game/Assets/Particles/NS_DirectionalImpact.NS_DirectionalImpact" (`Actor.GetActorBounds` DamagedActor true false)))
              (`NiagaraComponent.SetVariableFloat` _returnvalue "HitAngle" (.yaw (`KismetMathLibrary.FindLookAtRotation` (`Actor.K2_GetActorLocation` DamageCauser) (`Actor.K2_GetActorLocation` DamagedActor)))))
            (:`Is Not Valid`
              (goto _label_2))))))
    ; Duration
    (`KismetSystemLibrary.Delay` (`self.FlashDuration`))
    ; Undo material
    (`PrimitiveComponent.SetMaterial` (`self.FlashedComponent`) 0 (`self.OriginalMaterial`))))