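; Actor component that stores upgrades as saved gameplay effect classes and a map of integer stats.
; AddEffectstoSaved records each effect in both a lasting list and a pending list.
; ApplyLoadedEffects applies pending effects to the owner's Ability System Component and clears that list; its call in the event graph is disconnected.
; StatChange adds to existing stat entries only, truncating the result, and all three print debug messages.
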(event `Add Effects to Saved`
  (params (`Gameplay Effect` :type "GameplayEffect Class Reference (by ref)"))
  (`KismetArrayLibrary.Array_Add` (`self.Gameplay Effects Total Saved`) `Gameplay Effect`)
  (`KismetArrayLibrary.Array_Add` (`self.Gameplay Effects New To Be Applied`) `Gameplay Effect`)
  (`KismetSystemLibrary.PrintString` (`KismetTextLibrary.Conv_TextToString` (`|FormatText` "Loaded up {a}..." (`KismetSystemLibrary.GetClassDisplayName` `Gameplay Effect`))) true true (struct :`R` 0.049112 :`G` 1.0 :`B` 0.251657 :`A` 1.0) 12.0 "None"))

(fn `Apply Loaded Effects`
  (bind _returnvalue (`self.GetOwner`))
  (`/Engine/EditorBlueprintResources/StandardMacros.IsValid` (`self.GetOwner`)
    (:`Is Valid`
      (for _array_element (`self.Gameplay Effects New To Be Applied`)
        (bind _returnvalue_2 (`AbilitySystemComponent.BP_ApplyGameplayEffectToSelf` :`self` (`AbilitySystemBlueprintLibrary.GetAbilitySystemComponent` _returnvalue) :`GameplayEffectClass` _array_element))
        (bind _returnvalue_3 (`AbilitySystemBlueprintLibrary.GetActiveGameplayEffectStackCount` _returnvalue_2))
        (`KismetSystemLibrary.PrintString` (`KismetTextLibrary.Conv_TextToString` (`|FormatText` "Added {a} to {b}... stacks: {c}" (`KismetSystemLibrary.GetClassDisplayName` _array_element) _returnvalue _returnvalue_3)) true true (struct :`R` 0.049112 :`G` 1.0 :`B` 0.251657 :`A` 1.0) 12.0 "None"))
      (`KismetArrayLibrary.Array_Clear` (`self.Gameplay Effects New To Be Applied`)))))

(fn `Stat Change`
  (params (`Stat to Modify` :type "/Game/Game/Core/Blueprints/Data/Enumeration/E_Stats Enum" :default "NewEnumerator0") (`Add Value` :type "Float (double-precision)"))
  (bind _stat_to_modify (`local.Stat to Modify`))
  (bind (_value _returnvalue) (`BlueprintMapLibrary.Map_Find` (`self.Stats_Saved`) `Stat to Modify`))
  (bind _returnvalue_2 (`KismetMathLibrary.FTrunc` (+ _value (`local.Add Value`))))
  (if _returnvalue
    (`BlueprintMapLibrary.Map_Add` (`self.Stats_Saved`) _stat_to_modify _returnvalue_2)
    (`KismetSystemLibrary.PrintString` (`KismetTextLibrary.Conv_TextToString` (`|FormatText` "{a} new value: {b}" (`|GetEnumeratorNameAsString` _stat_to_modify) _returnvalue_2)) true true (struct :`R` 0.214241 :`G` 1.0 :`A` 1.0) 20.0)))