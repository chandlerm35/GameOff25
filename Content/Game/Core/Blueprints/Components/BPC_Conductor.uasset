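; BPC_Conductor is an actor component that relays music events from GI_GameInstance to its owning actor through its own dispatchers.
; It binds to the game instance's rhythm tempo event on BeginPlay or RebindEvents and re-broadcasts it.
; Beat and boss-move relay events exist, but their game-instance bindings are disconnected.
; UnbindFromMusicEvents clears every listener on the tempo dispatcher, including those of other objects.
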(event `RebindEvents`
  ;[0.284 0 1] Bind to music events on creation.
  (bind _asgi_game_instance (cast `/Game/Game/Core/GameInstance/GI_GameInstance` (`GameplayStatics.GetGameInstance`) :!label _label))
  (`|ExecutionSequence`
    (:`then_0`
      (add `/Game/Game/Core/GameInstance/GI_GameInstance.OnRhythm_Tempo` _asgi_game_instance (delegate `rhythm_tempo`)))))

(event `self.ReceiveBeginPlay`
  ;[0.284 0 1] Bind to music events on creation.
  (goto _label))

(event `rhythm_beat`
  ;[0.284 0 1] Bind to music events on creation.
  (`self.On_rhythm_beat`) ; Call this event on the actor that has this component
)

(event `rhythm_tempo`
  ;[0.284 0 1] Bind to music events on creation.
  (`self.On_rhythm_tempo`))

(event `boss_move` :!signature `self.On_boss_move`
  (params (MoveInt :type Integer))
  ;[0.284 0 1] Bind to music events on creation.
  (`self.On_boss_move` MoveInt))

(event `UnbindFromMusicEvents`
  ;[0.284 0 1] Unbind when done
  (bind _asgi_game_instance (cast `/Game/Game/Core/GameInstance/GI_GameInstance` (`GameplayStatics.GetGameInstance`)))
  (`|ExecutionSequence`
    (:`then_0`
      (clear `/Game/Game/Core/GameInstance/GI_GameInstance.OnRhythm_Tempo` _asgi_game_instance))))