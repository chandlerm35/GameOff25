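; SpawnPoint is a component that represents a spawn point belonging to a BP_SpawnPointBank actor.
; GetOwnerBank caches its owner as OwningBank when the owner's class is exactly BP_SpawnPointBank, so subclasses do not match.
; An invalid owner prints an on-screen error, while a valid owner of another class fails silently.
; The event graph holds no active logic, and nothing here calls GetOwnerBank.
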(fn `GetOwnerBank`
  (bind _returnvalue (`self.GetOwner`))
  (`/Engine/EditorBlueprintResources/StandardMacros.IsValid` _returnvalue
    (:`Is Valid`
      (if (== (`GameplayStatics.GetObjectClass` _returnvalue) "/Game/Game/Core/Blueprints/Actors/BP_SpawnPointBank.BP_SpawnPointBank_C")
        (bind _asbp_spawn_point_bank (cast `/Game/Game/Core/Blueprints/Actors/BP_SpawnPointBank` _returnvalue))
        (set `self.OwningBank` _asbp_spawn_point_bank)))
    (:`Is Not Valid`
      (`KismetSystemLibrary.PrintString` (`KismetTextLibrary.Conv_TextToString` (`|FormatText` (`KismetSystemLibrary.GetDisplayName` self) "{self} failed to find owning spawn bank")) true true (struct :`R` 1.0 :`G` 0.00584 :`A` 1.0) 30.0))))