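; Game state for cutscene levels that pushes a hex transition, spawns a post-process holder and plays credits music on BeginPlay.
; When the transition's end animation finishes, it messages the level script to begin the cutscene.
; It also tracks score, a movement lock and enemy manager waves, and pushes round-clear and gated player/boss death cut-in widgets.
; The timed desaturation fade is disconnected, as LoopStart is empty.
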(event `self.ReceiveBeginPlay`
  (`KismetSystemLibrary.DelayUntilNextTick`)
  (bind _returned_widget (`/Game/Game/Core/FunctionLibraries/BPFL_UI_FrequentFunctions2.Game_PushTransitionWidget` (`GameplayStatics.GetPlayerController` 0) "/Game/Game/Core/UI/Widgets/Widget_Transitions/UI_Transition_Hex.UI_Transition_Hex_C"))
  (set `self.Current Transition Widget` _returned_widget)
  (bind _returnvalue (`|SpawnActorFromClass` "/Game/Game/Core/Blueprints/Actors/BP_PostProcessWorld.BP_PostProcessWorld_C" (`KismetMathLibrary.MakeTransform` (0.0 0.0 0.0)) "Undefined" "MultiplyWithRoot" null null))
  (set `self.PostProcess_Holder` _returnvalue)
  (bind _is_streaming_completed_ (`/Game/Game/Core/FunctionLibraries/BPFL_Gameplay_FrequentFunctions.World_CheckIsStreamingCompleted`))
  (`KismetSystemLibrary.PrintString` (`KismetTextLibrary.Conv_TextToString` (`|FormatText` "Streaming completed... {a}" _is_streaming_completed_)) true true (struct :`R` 1.0 :`G` 0.070112 :`B` 0.220031 :`A` 1.0) 12.0)
  (bind _asui_transition_hex (cast `/Game/Game/Core/UI/Widgets/Widget_Transitions/UI_Transition_Hex` (`self.Current Transition Widget`)))
  (add `/Game/Game/Core/UI/Widgets/Widget_Transitions/UI_Transition_Hex.FinishedEndAnim` _asui_transition_hex (delegate `StartGame`))
  (`self.Loop Start`)
  (`/Game/Game/Core/FunctionLibraries/BPFL_FrequentFunctions.FMODPlayMusic` "/Game/FMOD/Events/Music/CreditsMusic.CreditsMusic"))

(event `StartGame`
  (bind _returnvalue (`GameplayStatics.GetActorOfClass` "/Script/Engine.LevelScriptActor"))
  (message `/Game/Game/Core/Blueprints/Data/Interface/BPI_LevelEvents.Ev_CallCutscene` _returnvalue))

(event `self.Fn_AddScoreToCurrentScore`
  (params (`Added Value` :type Integer))
  (set `self.CurrentScore` (`KismetMathLibrary.Clamp` (+ `Added Value` (`self.CurrentScore`)) 0 2147483647)))

(event `PlayerDeath`
  ; Player Death
  (`self.OnPlayerDeath`)
  (`KismetSystemLibrary.PrintString` "Gamestate called on player death" true true (struct :`G` 1.0 :`B` 0.145207 :`A` 1.0) 30.0 "GSPlayerDeath")
  (`/Engine/EditorBlueprintResources/StandardMacros.Gate` false :!label _label
    (:`Exit`
      (bind _returned_widget (`/Game/Game/Core/FunctionLibraries/BPFL_UI_FrequentFunctions2.Game_PushWidget` (`GameplayStatics.GetPlayerController` 0) "NewEnumerator0" "/Game/Game/Core/UI/Widgets/WBP_PlayerKill_CutIn.WBP_PlayerKill_CutIn_C"))
      (`|ExecutionSequence`
        (:`then_0`
          (goto _label :!via `Close`))
        (:`then_1`
          (add `CommonActivatableWidget.BP_OnWidgetDeactivated` _returned_widget (delegate `Bind_GameOver`)))))))

(event `Bind_GameOver`
  (goto _label :!via `Open`))

(event `Loop Start`
  ; POST PROCESS: Gradually lower Desaturation
)

(event `BossDeath`
  ; Boss Death
  (`self.OnBossDeath`)
  (`KismetSystemLibrary.PrintString` "Gamestate called on boss death" true true (struct :`G` 1.0 :`B` 0.145207 :`A` 1.0) 30.0 "GSBossDeath")
  (`/Engine/EditorBlueprintResources/StandardMacros.Gate` false :!label _label_2
    (:`Exit`
      (bind _returned_widget (`/Game/Game/Core/FunctionLibraries/BPFL_UI_FrequentFunctions2.Game_PushWidget` (`GameplayStatics.GetPlayerController` 0) "NewEnumerator0" "/Game/Game/Core/UI/Widgets/WBP_BossKill_CutIn.WBP_BossKill_CutIn_C"))
      (`|ExecutionSequence`
        (:`then_0`
          (goto _label_2 :!via `Close`))
        (:`then_1`
          (add `CommonActivatableWidget.BP_OnWidgetDeactivated` _returned_widget (delegate `Bind_KillScreen`)))))))

(event `Loop_PostProcess`
  (bind _weighted_blendable_value_local (`self.Weighted Blendable Value Local`))
  ; POST PROCESS: Gradually lower Desaturation
  (if (>= (`self.Weighted Blendable Value Local`) 0.0)
    (bind _output_get (set `self.Weighted Blendable Value Local` (`KismetMathLibrary.Lerp` _weighted_blendable_value_local (- _weighted_blendable_value_local 0.05) 1.5)))
    (`KismetMaterialLibrary.SetScalarParameterValue` "/Game/Game/Assets/Materials/MPC_DesaturateParams.MPC_DesaturateParams" "Intensity" _output_get)
    (else
      (`KismetSystemLibrary.K2_ClearAndInvalidateTimerHandle` (`self.Loop_PPM`)))))

(event `Bind_KillScreen`
  (goto _label_2 :!via `Open`))

(event `UpdateEnemyManager`
  (params (EnemyManager :type "/Game/Game/Core/Blueprints/Actors/BP_EnemyManager Object Reference"))
  ; Event Manager and event Dispatchers
  (clear `/Game/Game/Core/Blueprints/Actors/BP_EnemyManager.OnWaveCompleted` EnemyManager)
  (clear `/Game/Game/Core/Blueprints/Actors/BP_EnemyManager.OnWaveCompleted` EnemyManager)
  (clear `/Game/Game/Core/Blueprints/Actors/BP_EnemyManager.OnWaveUpdated` EnemyManager)
  (bind _output_get (set `self.CurrentEnemyManager` EnemyManager))
  (`/Engine/EditorBlueprintResources/StandardMacros.IsValid` _output_get
    (:`Is Valid`
      (add `/Game/Game/Core/Blueprints/Actors/BP_EnemyManager.OnWaveSpawned` _output_get (delegate `WaveSpawned`))
      (add `/Game/Game/Core/Blueprints/Actors/BP_EnemyManager.OnWaveCompleted` _output_get (delegate `WaveCompleted`))
      (add `/Game/Game/Core/Blueprints/Actors/BP_EnemyManager.OnWaveUpdated` _output_get (delegate `WaveUpdated`)))
    (:`Is Not Valid`
      (`KismetSystemLibrary.PrintString` "GameState has an invalid reference to the current enemy manager" true true (struct :`R` 1.0 :`B` 0.120697 :`A` 1.0) 30.0 "GameStateEnemyManagerInvalid"))))

(event `WaveSpawned`
  (params (MaxWaveSize :type Integer))
  ; Event Manager and event Dispatchers
  (bind _output_get (set `self.CurrentWaveMax` MaxWaveSize))
  (set `self.CurrentWaveRemaining` _output_get)
  (`/Engine/EditorBlueprintResources/StandardMacros.IncrementInt` (`self.WaveNumber`)))

(event `WaveUpdated`
  ; Event Manager and event Dispatchers
  (`/Engine/EditorBlueprintResources/StandardMacros.DecrementInt` (`self.CurrentWaveRemaining`)))

(event `WaveCompleted`
  ; Event Manager and event Dispatchers
  (`/Game/Game/Core/FunctionLibraries/BPFL_UI_FrequentFunctions2.Game_PushWidget` (`GameplayStatics.GetPlayerController` 0) "NewEnumerator0" "/Game/Game/Core/UI/Widgets/WBP_RoundClear.WBP_RoundClear_C"))

(event `self.Fn_DisableMovement`
  (params (`Disable?` :type Boolean))
  (set `self.DisableRotation` `Disable?`))

(fn `Fn_GetCurrentScore`
  (returns (`Current Score` :type Integer))
  (return (`self.CurrentScore`)))

(fn `Fn_GetInputInfo`
  (returns (`Disabled Movement?` :type Boolean))
  (return (`self.DisableRotation`)))

(fn `Fn_GetWaveAmount`
  (returns (Amount :type Integer) (MaxAmount :type Integer) (`Wave Number` :type Integer) (`Wave Max` :type Integer))
  (return (`self.CurrentWaveRemaining`) (`self.CurrentWaveMax`) (`self.WaveNumber`) 0))

(fn `Fn_GetWorldPostProcesses`
  (returns (`World Post Process Spawned` :type "/Game/Game/Core/Blueprints/Actors/BP_PostProcessWorld Object Reference"))
  (return (`self.PostProcess_Holder`)))

(fn `UserConstructionScript`)