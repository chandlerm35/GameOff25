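; BP_ArenaDoor is a double sliding arena door that locks and closes when its referenced boss encounter starts.
; Tick watches the boss's Started flag while unlocked, with no unlock path in this graph.
; Overlaps open it for combatants while unlocked, or for the boss under a "Boss" tag check.
; A timeline slides both panels, reversing when a combatant leaves and the player is not overlapping.
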(event `self.ReceiveTick`
  (params (DeltaSeconds :type "Float (single-precision)"))
  (if (`self.Unlocked`)
    (bind _output_get (set `self.Unlocked` (not (`/Game/Game/Core/Blueprints/Combatants/Enemy/BP_BossBase.Started` (`self.BossRef`)))))
    (if (not _output_get)
      (bind (_direction _openlerp) (`Timeline|OpenDoor` :!via `Reverse` :!label _label)
        (:`Update`
          (`SceneComponent.K2_SetRelativeLocation` (`self.LeftDoor`) (`KismetMathLibrary.MakeVector` -40.0 (`KismetMathLibrary.Lerp` -25.0 -75.0 _openlerp)) false false)
          (`SceneComponent.K2_SetRelativeLocation` (`self.RightDoor`) (`KismetMathLibrary.MakeVector` -40.0 (`KismetMathLibrary.Lerp` 25.0 75.0 _openlerp)) false false))))))

(event `self.ReceiveActorBeginOverlap`
  (params (OtherActor :type "Actor Object Reference"))
  (if (or (and (`GameplayStatics.ObjectIsA` OtherActor "/Game/Game/Core/Blueprints/Combatants/BP_CombatantBase.BP_CombatantBase_C") (`self.Unlocked`)) (and (== (`self.BossRef`) OtherActor) (== (`self.Tag`) "Boss") true))
    (goto _label)))

(event `self.ReceiveActorEndOverlap`
  (params (OtherActor :type "Actor Object Reference"))
  (if (and (`GameplayStatics.ObjectIsA` OtherActor "/Game/Game/Core/Blueprints/Combatants/BP_CombatantBase.BP_CombatantBase_C") (not (`KismetArrayLibrary.Array_Contains` (`self.GetOverlappingActors` "/Script/Engine.Pawn") (`GameplayStatics.GetPlayerPawn` 0))))
    (goto _label :!via `Reverse`)))

(fn `UserConstructionScript`)