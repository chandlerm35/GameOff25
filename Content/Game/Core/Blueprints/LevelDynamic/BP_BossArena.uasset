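; Boss arena actor that slides itself onscreen to the player camera's XY position at a fixed height when play begins.
; It spawns two arena doors sharing the boss reference, attached at the player and boss door points, the latter tagged Boss.
; A timeline, rate-scaled by distance and PlayerSpeed, moves only the Floor component, then teleports the actor there, resets the floor and calls ArenaFinished.
; The box overlap's boss check does nothing.
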(event `self.ReceiveBeginPlay`
  (bind _bossref (`self.BossRef`))
  (bind _target (`self.Target`))
  (bind _returnvalue (`|SpawnActorFromClass` "/Game/Game/Core/Blueprints/LevelDynamic/BP_ArenaDoor.BP_ArenaDoor_C" (`KismetMathLibrary.MakeTransform` (0.0 0.0 0.0) (struct) (1.0 1.2 1.0)) "Undefined" "MultiplyWithRoot" null _bossref "None" null))
  (`self.K2_AttachToComponent` _returnvalue (`self.PlayerDoor`) "None" "SnapToTarget" "SnapToTarget" "KeepWorld" true)
  (bind _returnvalue_2 (`|SpawnActorFromClass` "/Game/Game/Core/Blueprints/LevelDynamic/BP_ArenaDoor.BP_ArenaDoor_C" (`KismetMathLibrary.MakeTransform` (0.0 0.0 0.0) (struct) (1.0 1.2 1.0)) "Undefined" "MultiplyWithRoot" null _bossref "Boss" null))
  (`self.K2_AttachToComponent` _returnvalue_2 (`self.BossDoor`) "None" "SnapToTarget" "SnapToTarget" "KeepWorld" true)
  (bind _output_get (set `self.Target` (+ (* (`PlayerCameraManager.GetCameraLocation` (`GameplayStatics.GetPlayerCameraManager` 0)) (1.0 1.0 0.0)) (0.0 0.0 -100.0))))
  (`TimelineComponent.SetPlayRate` (`self.MoveOnscreen`) (/ 1.0 (* (`self.PlayerSpeed`) (/ (`KismetMathLibrary.VSize` (- (`self.K2_GetActorLocation`) _output_get)) 500.0))))
  (bind (_direction _lerp) (`Timeline|MoveOnscreen` :!via `PlayFromStart`)
    (:`Update`
      (`SceneComponent.K2_SetRelativeLocation` (`self.Floor`) (`KismetMathLibrary.VLerp` (0.0 0.0 0.0) (- _target (`self.K2_GetActorLocation`)) _lerp) false false))
    (:`Finished`
      (`self.K2_SetActorLocation` _target false true)
      (`SceneComponent.K2_SetRelativeLocation` (`self.Floor`) (0.0 0.0 0.0) false true)
      (`self.ArenaFinished`))))

(event `self.Box.OnComponentBeginOverlap`
  (params (OverlappedComponent :type "PrimitiveComponent Object Reference") (OtherActor :type "Actor Object Reference") (OtherComp :type "PrimitiveComponent Object Reference") (OtherBodyIndex :type Integer) (bFromSweep :type Boolean) (SweepResult :type "HitResult Structure (by ref)"))
  (if (== OtherActor (`self.BossRef`))
    _))

(fn `UserConstructionScript`)