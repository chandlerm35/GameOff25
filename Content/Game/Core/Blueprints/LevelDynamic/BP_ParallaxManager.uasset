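; Parallax manager that scrolls two scenery meshes, left and right, along negative X at a rate based on the square of PlayerSpeed.
; BeginPlay passes PlayerSpeed to the Cube's materials and starts a randomized, speed-scaled timer.
; PushObject recycles one mesh with a random model, side offset, yaw and flattened scale, then re-arms the timer.
; Side choice uses running selection counters as weights to keep left and right balanced.
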(event `self.ReceiveTick`
  (params (DeltaSeconds :type "Float (single-precision)"))
  (bind _returnvalue (`KismetMathLibrary.FMax` (`self.PlayerSpeed`) 1.0))
  (`SceneComponent.K2_AddRelativeLocation` (`self.ObjL`) (`KismetMathLibrary.MakeVector` (* DeltaSeconds (* _returnvalue _returnvalue) -1.0)) false false)
  (`SceneComponent.K2_AddRelativeLocation` (`self.ObjR`) (`KismetMathLibrary.MakeVector` (* DeltaSeconds (* _returnvalue _returnvalue) -1.0)) false false))

(event `self.ReceiveBeginPlay`
  (bind _playerspeed (`self.PlayerSpeed`))
  (`MeshComponent.SetScalarParameterValueOnMaterials` (`self.Cube`) "PlayerSpeed" (`self.PlayerSpeed`))
  (`KismetSystemLibrary.K2_SetTimerDelegate` (`|CreateDelegate` :!event `PushObject`) (/ (+ 100.0 (* (`KismetMathLibrary.RandomFloat`) 3.0) -1.5) _playerspeed _playerspeed) :!label _label))

(event `PushObject`
  (bind _returnvalue (/ (`KismetMathLibrary.RandomFloatInRange` 8.0 24.0) 30.0))
  (bind (_o _r) (`self.IncrementRandomInt` (`KismetMathLibrary.RandomBoolWithWeight` (/ (`self.RightSelection`) (`KismetMathLibrary.Conv_IntToDouble` (`KismetMathLibrary.Max` (+ (`self.LeftSelection`) (`self.RightSelection`)) 1))))))
  (bind _returnvalue_2 (select `bool` _r :`false` (`self.ObjL`) :`true` (`self.ObjR`)))
  (`SceneComponent.K2_SetRelativeLocation` _returnvalue_2 (`KismetMathLibrary.MakeVector` 50.0 (+ (* (`KismetMathLibrary.RandomFloat`) 10.0) (`KismetMathLibrary.SelectFloat` -25.0 25.0 _r)) 500.0) false false)
  (`StaticMeshComponent.SetStaticMesh` _returnvalue_2 (`|GetArrayItem` (`self.SpawnedObjects`) (`KismetMathLibrary.RandomIntegerInRange` 0 (`KismetArrayLibrary.Array_Length` (`self.SpawnedObjects`)))))
  (`SceneComponent.K2_SetRelativeRotation` _returnvalue_2 (`KismetMathLibrary.MakeRotator` 0.0 0.0 (* (`KismetMathLibrary.RandomFloat`) 360.0)) false false)
  (`SceneComponent.SetWorldScale3D` _returnvalue_2 (`KismetMathLibrary.MakeVector` _returnvalue _returnvalue 0.1))
  (goto _label))

(fn `IncrementRandomInt`
  (params (Random :type Boolean))
  (returns (O :type "Integer (by ref)") (R :type Boolean))
  (locals (LocalBool :type Boolean))
  (bind _localbool (`local.LocalBool`))
  (bind _output_get (set `local.LocalBool` Random))
  (if _output_get
    (bind _result (`/Engine/EditorBlueprintResources/StandardMacros.IncrementInt` (`self.LeftSelection`))
      (:`  `
        (return _result _localbool)))
    (else
      (bind _result_2 (`/Engine/EditorBlueprintResources/StandardMacros.IncrementInt` (`self.RightSelection`))
        (:`  `
          (return _result_2 _localbool))))))

(fn `UserConstructionScript`)