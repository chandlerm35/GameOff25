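; BP_PlayerGameplayTest is a player controller, apparently for gameplay testing, that sets up camera, input and HUD on BeginPlay.
; After camera setup and a short delay, it adds the IMC_Player Enhanced Input mapping, printing a message if the subsystem is invalid.
; It also initializes the basic HUD, then switches to game-only input with the cursor hidden.
; The pause action pushes the pause menu widget into a UI slot.
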(event `self.ReceiveBeginPlay`
  (bind _returnvalue (pcsubsystem `EnhancedInputLocalPlayerSubsystem` self))
  ; Beginplay
  (`|ExecutionSequence`
    (:`then_0`
      (`self.Set Up Camera`)
      (`KismetSystemLibrary.Delay` 0.5)
      (`/Engine/EditorBlueprintResources/StandardMacros.IsValid` _returnvalue
        (:`Is Valid`
          (`EnhancedInputSubsystemInterface.AddMappingContext` _returnvalue "/Game/Game/Core/Blueprints/PlayerControllers/Inputs/IMC_Player.IMC_Player" 0 (struct)))
        (:`Is Not Valid`
          (`KismetSystemLibrary.PrintString` "Not valid Local Input Player"))))
    (:`then_1`
      (`self.Ev_InitializeHUD` "/Game/Game/Core/UI/Widgets/WBP_HUD_Basic.WBP_HUD_Basic_C")
      (`KismetSystemLibrary.Delay` 0.1)
      (`WidgetBlueprintLibrary.SetInputMode_GameOnly` self true)
      (`/Game/Game/Core/FunctionLibraries/BPFL_UI_FrequentFunctions2.UI_ShowMouse_Cursor` false))))

(event `EnhancedInput|/Game/Game/Core/Blueprints/PlayerControllers/Inputs/Actions/Game/IA_Pause`
  (params (ActionValue :type "Vector2D Structure") (ElapsedSeconds :type "Float (double-precision)") (TriggeredSeconds :type "Float (double-precision)") (InputAction :type "InputAction Object Reference" :default "/Game/Game/Core/Blueprints/PlayerControllers/Inputs/Actions/Game/IA_Pause.IA_Pause"))
  (:`Started`
    (`/Game/Game/Core/FunctionLibraries/BPFL_UI_FrequentFunctions2.Game_PushWidget` self "NewEnumerator1" "/Game/Game/Core/UI/Widgets/WBP_PauseMenu.WBP_PauseMenu_C")))

(fn `UserConstructionScript`)