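; BP_PlayerTest is a player controller, apparently for testing, that sets up input, HUD and UI hooks.
; BeginPlay adds and registers the IMC_GameOffPlayer Enhanced Input context, initializes the basic HUD, then after short delays switches to game-only input with a hidden cursor.
; The pause action pushes the pause menu widget.
; Debug keys push warning and round-results widgets or add score, and possession prints the pawn's name.
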(event Input|EnhancedActionEvents|EnhancedInputActionIA_Pause
  (params (ActionValue :type Vector%202D%20Structure) (ElapsedSeconds :type Float%20%28double-precision%29) (TriggeredSeconds :type Float%20%28double-precision%29) (InputAction :type Input%20Action%20Object%20Reference :default "/Game/Game/Core/Blueprints/PlayerControllers/Inputs/Actions/Game/IA_Pause.IA_Pause"))
  (:Started
    (CallFunction|GamePushWidget self "NewEnumerator1" "/Game/Game/Core/UI/Widgets/WBP_PauseMenu.WBP_PauseMenu_C")))

(event EventPossess
  (params (PossessedPawn :type Pawn%20Object%20Reference))
  (|CallParentFunction PossessedPawn)
  (Development|PrintString (Utilities|GetDisplayName PossessedPawn) true true "(R=1.000000,G=0.708144,B=0.000000,A=1.000000)" 3e+01))

(event EventBeginPlay
  (bind _self self)
  (bind _returnvalue (PlayerController|LocalPlayerSubsystems|GetEnhancedInputLocalPlayerSubsystem _self))
  (Utilities|FlowControl|Sequence
    (:then_0
      ;[0.15 0.15 0.15 0.5] Beginplay
      (Utilities|FlowControl|Sequence
        (:then_0
          (Utilities|FlowControl|Delay 0.5)
          (Utilities|IsValid _returnvalue
            (:Is%20Valid
              (Input|AddMappingContext _returnvalue "/Game/Game/Core/Blueprints/PlayerControllers/Inputs/IMC_GameOffPlayer.IMC_GameOffPlayer" 0 "(bIgnoreAllPressedKeysUntilRelease=True,bForceImmediately=False,bNotifyUserSettings=False)")
              (bind _returnvalue_2 (Class|EnhancedInputUserSettings|RegisterInputMappingContext (Class|EnhancedInputSubsystemInterface|GetUserSettings _returnvalue) "/Game/Game/Core/Blueprints/PlayerControllers/Inputs/IMC_GameOffPlayer.IMC_GameOffPlayer"))
              (Development|PrintString (Utilities|String|ToString(Boolean) _returnvalue_2)))
            (:Is%20Not%20Valid
              (Development|PrintString "Not valid Local Input Player"))))
        (:then_1
          (CallFunction|EvInitializeHUD "/Game/Game/Core/UI/Widgets/WBP_HUD_Basic.WBP_HUD_Basic_C") ; debug unhooking
          (Utilities|FlowControl|Delay 0.1)
          (Input|SetInputModeGameOnly self true)
          (CallFunction|UIShowMouseCursor false))))
    (:then_1
      (if (Pawn|IsLocalPlayerController)
        (Input|AddMappingContext (PlayerController|LocalPlayerSubsystems|GetEnhancedInputLocalPlayerSubsystem) "/Game/Game/Core/Blueprints/PlayerControllers/Inputs/IMC_GameOffPlayer.IMC_GameOffPlayer" 0 "(bIgnoreAllPressedKeysUntilRelease=True,bForceImmediately=False,bNotifyUserSettings=False)")))))

(event Input|KeyboardEvents|DebugKey9
  (params (Key :type Key%20Structure :default "None") (ActionValue :type Input%20Action%20Value%20Structure))
  (:Released
    (CallFunction|GamePushWidget self "NewEnumerator0" "/Game/Game/Core/UI/Widgets/WBP_Warning.WBP_Warning_C")))

(event Input|KeyboardEvents|DebugKey7
  (params (Key :type Key%20Structure :default "None") (ActionValue :type Input%20Action%20Value%20Structure))
  (:Released
    (CallFunction|GamePushWidget self "NewEnumerator0" "/Game/Game/Core/UI/Widgets/WBP_RoundResults.WBP_RoundResults_C")))

(event Input|KeyboardEvents|DebugKey6
  (params (Key :type Key%20Structure :default "None") (ActionValue :type Input%20Action%20Value%20Structure))
  (:Released
    (CallFunction|GameAddtoCurrentScore 1000)))

(fn ConstructionScript)