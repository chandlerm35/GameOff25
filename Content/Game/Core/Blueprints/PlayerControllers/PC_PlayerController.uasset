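; PC_PlayerController is a player controller that sets up the player's HUD.
; EvInitializeHUD calls AddHUDElements, which creates WBP_UI_Base behind a DoOnce, stores it and adds it to the viewport.
; It then pushes the supplied HUD widget class into a UI slot through GamePushWidget.
; Getters for device name, player state, possessed actor and UI base are stubs returning no real data.
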(event `/Game/Blueprints/Data/Interface/BPI_Controller.Ev_InitializeHUD`
  (params (`HUD to Call` :type "CommonActivatableWidget Class Reference"))
  ; Set up HUD UI Base
  (`self.Add HUD Elements` `HUD to Call`))

(fn `Add HUD Elements`
  (params (`HUD Widget to Set` :type "CommonActivatableWidget Class Reference"))
  (`/Engine/EditorBlueprintResources/StandardMacros.DoOnce` false
    (:`Completed`
      (bind _returnvalue (`|CreateWidget` "/Game/Blueprints/UI/WBP_UI_Base.WBP_UI_Base_C" self))
      (bind _output_get (set `self.UIBaseRef` _returnvalue))
      (`UserWidget.AddToViewport` _output_get 0)
      (`/Game/Game/Core/FunctionLibraries/BPFL_UI_FrequentFunctions.Game_PushWidget` self "NewEnumerator0" (`local.HUD Widget to Set`)))))

(fn `Fn_GetDeviceName`
  (returns (`Device Name` :type Name))
  (return "None"))

(fn `Fn_GetPlayerState`
  (returns (`Controller Player State` :type "PlayerState Object Reference"))
  (return null))

(fn `Fn_GetPossessedActor`
  (returns (`Possessed Actor` :type "Actor Object Reference"))
  (return null))

(fn `Fn_GetUIBase`
  (returns (`WBP User Base Game` :type "/Game/Blueprints/UI/WBP_UI_Base Object Reference"))
  (return null))

(fn `UserConstructionScript`)