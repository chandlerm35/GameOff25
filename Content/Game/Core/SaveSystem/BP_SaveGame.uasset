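; Save game object that holds saved player scores and hands itself to saveable objects for saving and loading.
; SaveScores stores the passed scores and prints an on-screen debug message.
; SaveAllData and LoadDataRequested send save and load messages with itself as argument, so each object handles its own data.
; The file contains no slot write, and its event graph call to SaveAllData is unconnected.
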(event `Save Scores`
  (params (PlayerScoresSaved :type "Map of Name to Integer"))
  (set `self.PlayerScoresSaved` PlayerScoresSaved)
  (`KismetSystemLibrary.PrintString` null (`KismetTextLibrary.Conv_TextToString` (`|FormatText` "SaveGame {a} has saved PlayerScores" self)) true true (struct :`R` 1.0 :`G` 0.758925 :`A` 1.0) 12.0))

(fn `LoadDataRequested`
  (params (Requester :type "Object Object Reference"))
  (message `/Game/Game/Core/Interfaces/BPI_Saveable.LoadData` Requester self)
  (return))

(fn `SaveAllData`
  (params (SaveableObjects :type "Array of Object Object Reference"))
  (for _array_element SaveableObjects
    (message `/Game/Game/Core/Interfaces/BPI_Saveable.SaveData` _array_element self))
  (return))