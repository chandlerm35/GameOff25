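; BP_ConceptFloor is a concept floor actor that moves continuously along a looping path.
; Each Tick shifts the root by the loop-start-to-end vector scaled by delta time, with MoveTimeXY and MoveTimeZ acting as rate multipliers.
; When XY comes within tolerance of EndLocation, it teleports to the loop start's XY and the Z recorded by the construction script.
; The construction script also computes per-axis deltas, which Tick leaves unused.
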(event `self.ReceiveTick`
  (params (DeltaSeconds :type "Float (single-precision)"))
  (bind (_endlocation_x _endlocation_y) (`KismetMathLibrary.BreakVector` (`self.EndLocation`)))
  (bind _delta_seconds (`self.Delta Seconds`))
  (bind _movetimexy (`self.MoveTimeXY`))
  (bind (_startlocation_x _startlocation_y _startlocation_z) (`KismetMathLibrary.BreakVector` (`self.StartLocation`)))
  (bind (_loopstartlocation_x _loopstartlocation_y) (`KismetMathLibrary.BreakVector` (`self.LoopStartLocation`)))
  (bind (_returnvalue_x _returnvalue_y) (`KismetMathLibrary.BreakVector` (`SceneComponent.K2_GetComponentLocation` (`self.DefaultSceneRoot`))))
  (set `self.Delta Seconds` DeltaSeconds)
  ; Should calculate when the floor will be done instead
  (if (== (`KismetMathLibrary.MakeVector` _returnvalue_x _returnvalue_y) (`KismetMathLibrary.MakeVector` _endlocation_x _endlocation_y) :`ErrorTolerance` 10.0)
    (`SceneComponent.K2_SetWorldLocation` (`self.DefaultSceneRoot`) (`KismetMathLibrary.MakeVector` _loopstartlocation_x _loopstartlocation_y _startlocation_z) false true)
    (else
      (`SceneComponent.K2_SetWorldLocation` (`self.DefaultSceneRoot`) (+ (`SceneComponent.K2_GetComponentLocation` (`self.DefaultSceneRoot`)) (* (* (- (`self.EndLocation`) (`self.LoopStartLocation`)) (`KismetMathLibrary.MakeVector` _delta_seconds _delta_seconds _delta_seconds)) (`KismetMathLibrary.MakeVector` _movetimexy _movetimexy (`self.MoveTimeZ`)))) false false))))

(fn `UserConstructionScript`
  (bind (_endlocation_x _endlocation_y _endlocation_z) (`KismetMathLibrary.BreakVector` (`self.EndLocation`)))
  (bind (_loopstartlocation_x _loopstartlocation_y _loopstartlocation_z) (`KismetMathLibrary.BreakVector` (`self.LoopStartLocation`)))
  (set `self.StartLocation` (`SceneComponent.K2_GetComponentLocation` (`self.DefaultSceneRoot`)))
  (set `self.ChangeInX` (- _loopstartlocation_x _endlocation_x))
  (set `self.ChangeInY` (- _loopstartlocation_y _endlocation_y))
  (set `self.ChangeInZ` (- _loopstartlocation_z _endlocation_z)))