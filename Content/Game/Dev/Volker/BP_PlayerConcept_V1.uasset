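; Prototype player character with twin-stick controls and Gameplay Ability System (GAS) integration.
; Move input drives world-axis movement, while look input sets a target yaw that Tick interpolates toward, printing speed for debugging.
; BeginPlay grants a movement ability and two other abilities, each activated by its own input.
; An attribute listener sends normalized health to FMOD and signals death at zero, with T applying test damage.
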(event `self.ReceiveBeginPlay`
  (`self.SetupGas`))

(event `self.ReceiveTick`
  (params (DeltaSeconds :type "Float (single-precision)"))
  (`self.RotatePlayer`)
  (`KismetSystemLibrary.PrintString` (`KismetStringLibrary.Conv_DoubleToString` (`KismetMathLibrary.VSize` (`self.GetVelocity`))) true true (struct :`G` 1.0 :`B` 0.04046 :`A` 1.0) 2.0 "Movement"))

(event `EnhancedInput|/Game/Game/Core/Blueprints/PlayerControllers/Inputs/Actions/Game/IA_Move`
  (params (ActionValue :type "Vector2D Structure") (ElapsedSeconds :type "Float (double-precision)") (TriggeredSeconds :type "Float (double-precision)") (InputAction :type "InputAction Object Reference" :default "/Game/Game/Core/Blueprints/PlayerControllers/Inputs/Actions/Game/IA_Move.IA_Move"))
  (:`Triggered`
    (`self.Move` ActionValue_X ActionValue_Y)))

(event `EnhancedInput|/Game/Game/Core/Blueprints/PlayerControllers/Inputs/Actions/Game/IA_Look`
  (params (ActionValue :type "Vector2D Structure") (ElapsedSeconds :type "Float (double-precision)") (TriggeredSeconds :type "Float (double-precision)") (InputAction :type "InputAction Object Reference" :default "/Game/Game/Core/Blueprints/PlayerControllers/Inputs/Actions/Game/IA_Look.IA_Look"))
  (:`Triggered`
    (if (`self.LookEnabled`)
      (`self.StickAim` ActionValue_X ActionValue_Y))))

(event `EnhancedInput|/Game/Game/Core/Blueprints/PlayerControllers/Inputs/Actions/Game/IA_MovementAbility`
  (params (ActionValue :type Boolean) (ElapsedSeconds :type "Float (double-precision)") (TriggeredSeconds :type "Float (double-precision)") (InputAction :type "InputAction Object Reference" :default "/Game/Game/Core/Blueprints/PlayerControllers/Inputs/Actions/Game/IA_MovementAbility.IA_MovementAbility"))
  (:`Triggered`
    (`AbilitySystemComponent.TryActivateAbilityByClass` (`self.AbilitySystemComponent`) (`self.MovementAbility`) true)))

(event `EnhancedInput|/Game/Game/Core/Blueprints/PlayerControllers/Inputs/Actions/Game/IA_Ablity1`
  (params (ActionValue :type Boolean) (ElapsedSeconds :type "Float (double-precision)") (TriggeredSeconds :type "Float (double-precision)") (InputAction :type "InputAction Object Reference" :default "/Game/Game/Core/Blueprints/PlayerControllers/Inputs/Actions/Game/IA_Ablity1.IA_Ablity1"))
  (:`Triggered`
    (`AbilitySystemComponent.TryActivateAbilityByClass` (`self.AbilitySystemComponent`) (`self.Ability1`) true)))

(event `EnhancedInput|/Game/Game/Core/Blueprints/PlayerControllers/Inputs/Actions/Game/IA_Ablity2`
  (params (ActionValue :type Boolean) (ElapsedSeconds :type "Float (double-precision)") (TriggeredSeconds :type "Float (double-precision)") (InputAction :type "InputAction Object Reference" :default "/Game/Game/Core/Blueprints/PlayerControllers/Inputs/Actions/Game/IA_Ablity2.IA_Ablity2"))
  (:`Triggered`
    (`AbilitySystemComponent.TryActivateAbilityByClass` (`self.AbilitySystemComponent`) (`self.Ability2`) true)))

(event `SetupGas`
  (`self.AddBaseAbilities`)
  (`self.HandleDamageTaken`)
  (`self.GASSetup`))

(event `HandleDamageTaken`
  ; FMOD gets health as percentage 0 - 1.0
  (bind (_asynctaskproxy _attribute _newvalue) (`AbilityAsync_WaitAttributeChanged.WaitForAttributeChanged` null (struct :`AttributeName` "Health" :`Attribute` "/Script/GameOff25.BasicAttributeSet:Health" :`AttributeOwner` "/Script/CoreUObject.Class'/Script/GameOff25.BasicAttributeSet'"))
    (:`Changed`
      (`FMODBlueprintStatics.SetGlobalParameterByName` "PlayerHealth" (/ _newvalue (`.ReturnValue` (`AbilitySystemBlueprintLibrary.GetFloatAttributeFromAbilitySystemComponent` (`self.AbilitySystemComponent`) (struct :`AttributeName` "MaxHealth" :`Attribute` "/Script/GameOff25.BasicAttributeSet:MaxHealth" :`AttributeOwner` "/Script/CoreUObject.Class'/Script/GameOff25.BasicAttributeSet'")))))
      (if (<= (`.ReturnValue` (`AbilitySystemBlueprintLibrary.GetFloatAttributeFromAbilitySystemComponent` (`self.AbilitySystemComponent`) (struct :`AttributeName` "Health" :`Attribute` "/Script/GameOff25.BasicAttributeSet:Health" :`AttributeOwner` "/Script/CoreUObject.Class'/Script/GameOff25.BasicAttributeSet'"))) 0.0)
        (`self.OnDeath`)))))

(event `Key|T`
  (params (Key :type "Key Structure"))
  (:`Pressed`
    (bind _returnvalue (`AbilitySystemBlueprintLibrary.MakeSpecHandleByClass` "/Game/Game/Core/Blueprints/Combatants/Abilities/Effects/GE_DamageInstant.GE_DamageInstant_C"))
    (bind _returnvalue_2 (`AbilitySystemBlueprintLibrary.AssignTagSetByCallerMagnitude` _returnvalue (struct :`TagName` "Data.Damage") -10.0))
    (`AbilitySystemComponent.BP_ApplyGameplayEffectSpecToSelf` (`self.AbilitySystemComponent`) _returnvalue_2)))

(fn `AddBaseAbilities`
  (`AbilitySystemComponent.K2_GiveAbility` (`self.AbilitySystemComponent`) (`self.MovementAbility`) 0 -1)
  (`AbilitySystemComponent.K2_GiveAbility` (`self.AbilitySystemComponent`) (`self.Ability1`) 0 -1)
  (`AbilitySystemComponent.K2_GiveAbility` (`self.AbilitySystemComponent`) (`self.Ability2`) 0 -1))

(fn `Aim`
  (params (`X Axis` :type "Float (single-precision)") (`Y Axis` :type "Float (double-precision)"))
  (`self.AddControllerYawInput` `X Axis`)
  (`self.AddControllerPitchInput` `Y Axis`))

(fn `Move`
  (params (`X Axis` :type "Float (double-precision)") (`Y Axis` :type "Float (double-precision)"))
  (`self.AddMovementInput` (0.0 1.0 0.0) `X Axis`)
  (`self.AddMovementInput` (1.0 0.0 0.0) `Y Axis`))

(fn `RotatePlayer`
  (locals (CurrentRotation :type "Rotator Structure" :default (struct)))
  (bind (_currentrotation_roll _currentrotation_pitch _currentrotation_yaw) (`KismetMathLibrary.BreakRotator` (`local.CurrentRotation`)))
  (bind (_currentrotation_roll_2 _currentrotation_pitch_2) (`KismetMathLibrary.BreakRotator` (`local.CurrentRotation`)))
  (bind (_returnvalue_roll _returnvalue_pitch _returnvalue_yaw) (`KismetMathLibrary.BreakRotator` (`KismetMathLibrary.RInterpTo` (`local.CurrentRotation`) (`KismetMathLibrary.MakeRotator` _currentrotation_roll_2 _currentrotation_pitch_2 (`self.Target Rotation`)) (`GameplayStatics.GetWorldDeltaSeconds`) (`self.TurnSpeed`))))
  (set `local.CurrentRotation` (`self.K2_GetActorRotation`))
  (if (not (`KismetMathLibrary.NearlyEqual_FloatFloat` _currentrotation_yaw (`self.Target Rotation`) 0.5))
    (`self.K2_SetActorRotation` (`KismetMathLibrary.MakeRotator` _returnvalue_roll _returnvalue_pitch _returnvalue_yaw))))

(fn `StickAim`
  (params (`Axis X` :type "Float (double-precision) (by ref)") (`Axis Y` :type "Float (double-precision)"))
  (bind _result (`/Engine/EditorBlueprintResources/StandardMacros.NegateFloat` `Axis X`)
    (:`  `
      (set `self.Target Rotation` (`KismetMathLibrary.DegAtan2` `Axis Y` _result)))))

(fn `UserConstructionScript`
  (`parent.UserConstructionScript`))