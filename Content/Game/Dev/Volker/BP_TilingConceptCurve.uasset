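; Prototype looping mover that slides the actor along the straight vector from a loop start to a loop end and teleports it back, apparently for a tiling concept.
; The construction script derives the loop duration from move speed and scales the first lap by the spawn point's distance to the loop end.
; Tick advances position and timer, carrying timer overshoot into the next lap to recover from lag spikes.
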(event `self.ReceiveTick`
  (params (DeltaSeconds :type "Float (single-precision)"))
  (set `self.Delta Seconds` DeltaSeconds)
  (if (`self.ShouldLoop`)
    (`SceneComponent.K2_SetWorldLocation` (`self.DefaultSceneRoot`) (`self.LoopStartLocation`) false true)
    (`self.IterateMoveTimer` (`self.Delta Seconds`))
    (else
      (`SceneComponent.K2_SetWorldLocation` (`self.DefaultSceneRoot`) (`self.GetNewLocation`) false false)
      (`self.IterateMoveTimer` (`self.Delta Seconds`)))))

(event `self.StaticMesh.OnComponentBeginOverlap`
  (params (OverlappedComponent :type "PrimitiveComponent Object Reference") (OtherActor :type "Actor Object Reference") (OtherComp :type "PrimitiveComponent Object Reference") (OtherBodyIndex :type Integer) (bFromSweep :type Boolean) (SweepResult :type "HitResult Structure (by ref)")))

(fn `GetFirstLoopDuration`
  (returns (MoveTime :type "Float (double-precision)"))
  (return (* (/ (`KismetMathLibrary.VSize` (- (`self.SpawnLocation`) (`self.LoopEndLocation`))) (`KismetMathLibrary.VSize` (- (`self.LoopStartLocation`) (`self.LoopEndLocation`)))) (`self.LoopDuration`))))

(fn `GetNewLocation`
  (returns (ReturnValue :type "Vector Structure"))
  (return (+ (`SceneComponent.K2_GetComponentLocation` (`self.DefaultSceneRoot`)) (* (* (- (`self.LoopEndLocation`) (`self.LoopStartLocation`)) (`self.Delta Seconds`)) (`self.MoveSpeed`)))))

(fn `IterateMoveTimer`
  (params (DeltaTime :type "Float (double-precision)"))
  (set `self.MoveTimer` (+ (`self.MoveTimer`) DeltaTime)))

(fn `ShouldLoop`
  (returns (ReturnValue :type Boolean))
  (locals (Output :type Boolean))
  (if (and (>= (`self.MoveTimer`) (`self.FirstLoopDuration`)) (`self.IsFirstLoop`))
    (set `self.IsFirstLoop` false)
    ;[0.15 0.15 0.15 0.5 14] Overshoot Correction (Recovers from Lag spikes)
    (set `self.MoveTimer` (- (`self.MoveTimer`) (`self.FirstLoopDuration`)))
    (set `local.Output` true)
    (elif (and (>= (`self.MoveTimer`) (`self.LoopDuration`)) (not (`self.IsFirstLoop`)))
      (set `self.MoveTimer` (- (`self.MoveTimer`) (`self.LoopDuration`)))
      (set `local.Output` true)
      (else
        (set `local.Output` false))))
  (return (`local.Output`)))

(fn `UserConstructionScript`
  (bind (_loopendlocation_x _loopendlocation_y _loopendlocation_z) (`KismetMathLibrary.BreakVector` (`self.LoopEndLocation`)))
  (bind (_loopstartlocation_x _loopstartlocation_y _loopstartlocation_z) (`KismetMathLibrary.BreakVector` (`self.LoopStartLocation`)))
  (set `self.SpawnLocation` (`SceneComponent.K2_GetComponentLocation` (`self.DefaultSceneRoot`)))
  (set `self.ChangeInX` (- _loopstartlocation_x _loopendlocation_x))
  (set `self.ChangeInY` (- _loopstartlocation_y _loopendlocation_y))
  (set `self.ChangeInZ` (- _loopstartlocation_z _loopendlocation_z))
  (set `self.LoopDuration` (/ 1.0 (`self.MoveSpeed`)))
  (bind _movetime (`self.GetFirstLoopDuration`))
  (set `self.FirstLoopDuration` _movetime))